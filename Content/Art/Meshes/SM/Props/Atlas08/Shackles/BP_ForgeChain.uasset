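; BP_ForgeChain is a forge chain prop that animates an instanced static mesh along its local Z axis.
; The construction script sets a direction multiplier from IsDown, so the chain travels either up or down.
; On BeginPlay a timeline drives the mesh's relative height, then restarts once from the beginning after a configurable delay.
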(event `self.ReceiveBeginPlay`
  (`|ExecutionSequence`
    (:`then_0`
      (bind (_direction _newtrack_0) (`Timeline|Timeline` :!via `PlayFromStart` :!label _label)
        (:`Update`
          (`SceneComponent.K2_SetRelativeLocation` (`self.InstancedStaticMesh`) (`KismetMathLibrary.MakeVector` (.x (`KismetMathLibrary.MakeVector` 0.0 0.0 (* _newtrack_0 10.0))) (.y (`KismetMathLibrary.MakeVector` 0.0 0.0 (* _newtrack_0 10.0))) (* (.z (`KismetMathLibrary.MakeVector` 0.0 0.0 (* _newtrack_0 10.0))) (`self.Scale`))) false false))))
    (:`then_1`
      (`KismetSystemLibrary.Delay` (`self.Delay`))
      (`/Engine/EditorBlueprintResources/StandardMacros.DoOnce` false
        (:`Completed`
          (goto _label :!via `PlayFromStart`))))))

(fn `UserConstructionScript`
  (if (`self.IsDown?`)
    (set `self.Scale` -1.0)
    (else
      (set `self.Scale` 1.0))))