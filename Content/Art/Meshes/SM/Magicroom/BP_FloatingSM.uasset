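; BP_FloatingSM is a decorative floating mesh actor that bobs and rotates, with an optional spectral look.
; The construction script gives each axis a random scale from a seeded stream, re-seeded when Randomization is on.
; On BeginPlay, Spectral applies a dynamic Fresnel material with random start point and speed, slower for meshes with larger X scale.
; After a random delay that staggers instances, two timelines drive relative location and rotation.
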(event `self.ReceiveBeginPlay`
  (bind _dynamicmaterial (`self.DynamicMaterial`))
  (bind _relativescale3d_x (`KismetMathLibrary.BreakVector` (`SceneComponent.RelativeScale3D` (`self.StaticMesh`))))
  (`|ExecutionSequence`
    (:`then_0`
      (if (`self.Spectral?`)
        (bind _returnvalue (`KismetMaterialLibrary.CreateDynamicMaterialInstance` "/Game/Art/Materials/MasterMaterials/MM_Fresnel.MM_Fresnel"))
        (bind _output_get (set `self.DynamicMaterial` _returnvalue))
        (`PrimitiveComponent.SetMaterial` (`self.StaticMesh`) 0 _output_get)
        (`MaterialInstanceDynamic.SetScalarParameterValue` (`self.DynamicMaterial`) "StartingPoint" (`KismetMathLibrary.RandomFloatInRange` 0.0 5.0))
        (if (> _relativescale3d_x 1.3)
          (`MaterialInstanceDynamic.SetScalarParameterValue` _dynamicmaterial "Speed" (`KismetMathLibrary.RandomFloatInRange` 0.1 0.5))
          (else
            (`MaterialInstanceDynamic.SetScalarParameterValue` _dynamicmaterial "Speed" (`KismetMathLibrary.RandomFloatInRange` 0.5 1.0))))))
    (:`then_1`
      (`KismetSystemLibrary.Delay` (`KismetMathLibrary.RandomFloatInRange` 0.0 2.0))
      (`self.Animation`))))

(event `Animation`
  (bind _staticmesh (`self.StaticMesh`))
  (`|ExecutionSequence`
    (:`then_0`
      (bind (_direction _float) (`Timeline|TranslateSM` :!via `PlayFromStart`)
        (:`Update`
          (`SceneComponent.K2_SetRelativeLocation` _staticmesh _float false false))))
    (:`then_1`
      (bind (_direction_2 _skullrotation) (`Timeline|RotationSM` :!via `PlayFromStart`)
        (:`Update`
          (`SceneComponent.K2_SetRelativeRotation` _staticmesh (`KismetMathLibrary.MakeRotator` (.x _skullrotation) (.y _skullrotation) (.z _skullrotation)) false false))))))

(fn `UserConstructionScript`
  (bind _returnvalue (`KismetMathLibrary.RandomFloatInRangeFromStream` (`self.Seed`) 0.5 2.0))
  (if (`self.Randomization`)
    (`KismetMathLibrary.SeedRandomStream` (`self.Seed`)))
  (`SceneComponent.SetRelativeScale3D` (`self.StaticMesh`) (`KismetMathLibrary.MakeVector` _returnvalue _returnvalue _returnvalue)))