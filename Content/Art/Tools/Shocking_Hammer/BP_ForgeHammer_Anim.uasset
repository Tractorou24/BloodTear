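; Animated forge hammer prop that continuously swings two hammers with a glowing emissive and a timed Niagara effect.
; On BeginPlay it creates one dynamic material from the atlas hammer material, shared by both meshes, and starts the animation.
; A timeline drives both pivots' pitch and the emissive power, restarting the cycle when finished.
; Each cycle also activates and later deactivates Niagara through fixed delays running alongside the timeline.
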(event `self.ReceiveBeginPlay`
  (bind _returnvalue (`KismetMaterialLibrary.CreateDynamicMaterialInstance` "/Game/Art/Materials/InstancedMaterials/Forge/AtlasHammer/MI_AtlasHammer.MI_AtlasHammer" "AtlasHammer_Emmisive"))
  (bind _output_get (set `self.DynamicMaterial` _returnvalue))
  (`PrimitiveComponent.SetMaterial` (`self.SM_Hammer01`) 0 _output_get)
  (`PrimitiveComponent.SetMaterial` (`self.SM_Hammer02`) 0 _output_get)
  (`self.Start_AnimationHammer`))

(event `Start_AnimationHammer`
  (bind _niagara (`self.Niagara`))
  (`|ExecutionSequence`
    (:`then_0`
      (bind (_direction _hammer01 _hammer02 _hammeremmisive) (`Timeline|Timeline` :!via `PlayFromStart`)
        (:`Update`
          (`SceneComponent.K2_SetRelativeRotation` (`self.PivotHammer01`) (`KismetMathLibrary.MakeRotator` 0.0 _hammer01) false false)
          (`SceneComponent.K2_SetRelativeRotation` (`self.PivotHammer02`) (`KismetMathLibrary.MakeRotator` 0.0 _hammer02) false false)
          (`MaterialInstanceDynamic.SetScalarParameterValue` (`self.DynamicMaterial`) "EmissivePower" _hammeremmisive))
        (:`Finished`
          (`self.Start_AnimationHammer`))))
    (:`then_1`
      (`KismetSystemLibrary.Delay` 0.9)
      (`ActorComponent.Activate` _niagara false)
      (`KismetSystemLibrary.Delay` 1.5)
      (`ActorComponent.Deactivate` _niagara))))

(fn `UserConstructionScript`)