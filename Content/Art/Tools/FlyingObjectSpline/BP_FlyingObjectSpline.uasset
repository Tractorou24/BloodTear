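; Art tool actor that flies a mesh along its spline, wrapping to the start when it passes the end.
; Tick advances distance by a speed value and aligns the mesh to the spline with a yaw offset.
; When Spectral is set, BeginPlay applies a dynamic Fresnel material with randomized start and flicker speed.
; That branch also starts a timeline that modulates the movement speed.
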(event `self.ReceiveBeginPlay`
  (bind _dynamicmaterial (`self.DynamicMaterial`))
  (if (`self.Spectral`)
    (bind _returnvalue (`KismetMaterialLibrary.CreateDynamicMaterialInstance` "/Game/Art/Materials/MasterMaterials/MM_Fresnel.MM_Fresnel"))
    (bind _output_get (set `self.DynamicMaterial` _returnvalue))
    (`PrimitiveComponent.SetMaterial` (`self.SM_Object`) 0 _output_get)
    (`MaterialInstanceDynamic.SetScalarParameterValue` _dynamicmaterial "StartingPoint" (`KismetMathLibrary.RandomFloatInRange` 0.0 5.0))
    (`MaterialInstanceDynamic.SetScalarParameterValue` _dynamicmaterial "Speed" (`KismetMathLibrary.RandomFloatInRange` (`self.SpectralFlickSpeed_Min`) (`self.SpectralFlickSpeed_Max`)))
    (`self.SpeedVariation`)))

(event `SpeedVariation`
  (bind (_direction _speedmultiplier) (`Timeline|Timeline` :!via `PlayFromStart`)
    (:`Update`
      (set `self.MovingSpeedMultiplied` (* (`self.MovingSpeed`) _speedmultiplier)))))

(event `self.ReceiveTick`
  (params (DeltaSeconds :type "Float (single-precision)"))
  (bind _returnvalue (`SplineComponent.GetTransformAtDistanceAlongSpline` (`self.Spline`) (`self.DistanceAlongSpline`) "Local" false))
  (set `self.DistanceAlongSpline` (+ (* DeltaSeconds (`self.MovingSpeedMultiplied`)) (`self.DistanceAlongSpline`)))
  (`SceneComponent.K2_SetRelativeTransform` (`self.SM_Object`) (`KismetMathLibrary.MakeTransform` (.location _returnvalue) (`KismetMathLibrary.MakeRotator` (.roll (.rotation _returnvalue)) (.pitch (.rotation _returnvalue)) (+ (.yaw (.rotation _returnvalue)) -90.0))) false false)
  (if (> (`self.DistanceAlongSpline`) (`SplineComponent.GetSplineLength` (`self.Spline`)))
    (set `self.DistanceAlongSpline` 0.0)))

(fn `UserConstructionScript`)