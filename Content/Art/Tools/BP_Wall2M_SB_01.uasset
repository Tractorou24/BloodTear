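; Modular wall piece that procedurally varies its look from a seeded random stream.
; The construction script groups components into arrays, optionally reseeds when Randomize is set, then runs Setup; the RandomSeed event also rerolls and rebuilds.
; Setup randomizes stone block visibility and Y scale on both faces, picks meshes and scales for under-walls and ground volumes, and picks an upper wall mesh with a possible 180-degree flip.
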(event `RandomSeed`
  (set `self.Seed` (`KismetMathLibrary.MakeRandomStream` (`KismetMathLibrary.RandomInteger` 9999)))
  (`self.Setup`))

(fn `Setup`
  (bind _seed (`self.Seed`))
  (bind _percentageofstonevisible (`self.PercentageOfStoneVisible`))
  (bind _minimumscale_stoneblocks (`self.MinimumScale_StoneBlocks`))
  (bind _maximumscale_stoneblocks (`self.MaximumScale_StoneBlocks`))
  (bind _upwall (`self.UpWall`))
  (bind _returnvalue (`KismetMathLibrary.RandomFloatInRangeFromStream` (`self.Seed`) (`self.MinimumScale_GroundVolume`) (`self.MaximumScale_GroundVolume`)))
  (`|ExecutionSequence`
    (:`then_0`
      (for _array_element (`self.Face01_StoneBlocks`)
        (`SceneComponent.SetVisibility` _array_element (`KismetMathLibrary.RandomBoolWithWeightFromStream` _seed _percentageofstonevisible) false)
        (`SceneComponent.SetRelativeScale3D` _array_element (`KismetMathLibrary.MakeVector` 1.0 (`KismetMathLibrary.RandomFloatInRangeFromStream` _seed _minimumscale_stoneblocks _maximumscale_stoneblocks) 1.0))))
    (:`then_1`
      (for _array_element_2 (`self.Face02_StoneBlocks`)
        (`SceneComponent.SetVisibility` _array_element_2 (`KismetMathLibrary.RandomBoolWithWeightFromStream` _seed _percentageofstonevisible) false)
        (`SceneComponent.SetRelativeScale3D` _array_element_2 (`KismetMathLibrary.MakeVector` 1.0 (`KismetMathLibrary.RandomFloatInRangeFromStream` _seed _minimumscale_stoneblocks _maximumscale_stoneblocks) 1.0))))
    (:`then_2`
      (for _array_element_3 (`self.UndWalls50`)
        (`StaticMeshComponent.SetStaticMesh` _array_element_3 (`|GetArrayItem` (`self.UndWall50_Data`) (`KismetMathLibrary.RandomIntegerInRangeFromStream` (`self.Seed`) 0 (- (`KismetArrayLibrary.Array_Length` (`self.UndWall50_Data`)) 1))))
        (`SceneComponent.SetRelativeScale3D` _array_element_3 (`KismetMathLibrary.MakeVector` 1.0 (`KismetMathLibrary.RandomFloatInRangeFromStream` (`self.Seed`) (`self.MinimumScale_UndWall`) (`self.MaximumScale_UndWall`)) 1.0))))
    (:`then_3`
      (for _array_element_4 (`self.GroundVolumes`)
        (`StaticMeshComponent.SetStaticMesh` _array_element_4 (`|GetArrayItem` (`self.GroundVolume_Data`) (`KismetMathLibrary.RandomIntegerInRangeFromStream` (`self.Seed`) 0 (- (`KismetArrayLibrary.Array_Length` (`self.GroundVolume_Data`)) 1))))
        (`SceneComponent.SetRelativeScale3D` _array_element_4 (`KismetMathLibrary.MakeVector` 1.0 _returnvalue _returnvalue))))
    (:`then_4`
      (`StaticMeshComponent.SetStaticMesh` (`self.UpWall`) (`|GetArrayItem` (`self.UpWalls_Data`) (`KismetMathLibrary.RandomIntegerInRangeFromStream` (`self.Seed`) 0 (- (`KismetArrayLibrary.Array_Length` (`self.UpWalls_Data`)) 1))))
      (if (`KismetMathLibrary.RandomBoolFromStream` (`self.Seed`))
        (`SceneComponent.K2_SetRelativeLocation` _upwall (200.0 0.0 260.0) false false)
        (`SceneComponent.K2_SetRelativeRotation` _upwall (`KismetMathLibrary.MakeRotator` 0.0 0.0 180.0) false false)))))

(fn `UserConstructionScript`
  (set `self.Face01_StoneBlocks` (`|MakeArray` (`self.Face01_Stone01`) (`self.Face01_Stone02`) (`self.Face01_Stone03`) (`self.Face01_Stone04`) (`self.Face01_Stone05`) (`self.Face01_Stone06`) (`self.Face01_Stone07`) (`self.Face01_Stone08`) (`self.Face01_Stone09`) (`self.Face01_Stone10`) (`self.Face01_Stone11`) (`self.Face01_Stone12`) (`self.Face01_Stone13`) (`self.Face01_Stone14`) (`self.Face01_Stone15`) (`self.Face01_Stone16`) (`self.Face01_Stone17`) (`self.Face01_Stone18`) (`self.Face01_Stone19`) (`self.Face01_Stone20`)))
  (set `self.Face02_StoneBlocks` (`|MakeArray` (`self.Face02_Stone01`) (`self.Face02_Stone02`) (`self.Face02_Stone03`) (`self.Face02_Stone04`) (`self.Face02_Stone05`) (`self.Face02_Stone06`) (`self.Face02_Stone07`) (`self.Face02_Stone08`) (`self.Face02_Stone09`) (`self.Face02_Stone10`) (`self.Face02_Stone11`) (`self.Face02_Stone12`) (`self.Face02_Stone13`) (`self.Face02_Stone14`) (`self.Face02_Stone15`) (`self.Face02_Stone16`) (`self.Face02_Stone17`) (`self.Face02_Stone18`) (`self.Face02_Stone19`) (`self.Face02_Stone20`)))
  (set `self.UndWalls50` (`|MakeArray` (`self.UndWall50_01`) (`self.UndWall50_02`)))
  (set `self.GroundVolumes` (`|MakeArray` (`self.GroundVolume_01`) (`self.GroundVolume_02`) (`self.GroundVolume_03`)))
  (if (`self.Randomize`)
    (`KismetMathLibrary.SetRandomStreamSeed` (`self.Seed`) (`KismetMathLibrary.RandomInteger` 9999)))
  (`self.Setup`))