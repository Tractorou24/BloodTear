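; BP_BedChain is an art tool actor that builds a chain of meshes along a spline in its construction script.
; It adds one spline mesh per section length, optionally taken from actor Y scale, and either drops or keeps the partial last section.
; Sections overlap slightly, and their tangents come from clamped spline positions rather than spline tangents.
; Start and end meshes are moved to the first and last spline points, without rotation.
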(fn `Get_End_Pos/Tangent`
  (params (Index :type Integer))
  (returns (Position :type "Vector Structure") (Tangent :type "Vector Structure"))
  (bind _spline (`self.Spline`))
  (bind _returnvalue (* (+ Index 1) (`self.SectionLenght`)))
  (return (`SplineComponent.GetLocationAtDistanceAlongSpline` _spline (- _returnvalue -3.0) "Local") (`KismetMathLibrary.ClampVectorSize` (`SplineComponent.GetLocationAtDistanceAlongSpline` _spline _returnvalue "Local") 0.0 (`self.SectionLenght`))))

(fn `get_Start_Pos /Tangent`
  (params (Index :type Integer))
  (returns (Position :type "Vector Structure") (Tangent :type "Vector Structure"))
  (bind _spline (`self.Spline`))
  (bind _returnvalue (* Index (`self.SectionLenght`)))
  (return (`SplineComponent.GetLocationAtDistanceAlongSpline` _spline _returnvalue "Local") (`KismetMathLibrary.ClampVectorSize` (`SplineComponent.GetLocationAtDistanceAlongSpline` _spline _returnvalue "Local") 0.0 (`self.SectionLenght`))))

(fn `Set_Start_End_Meshes`
  (bind _spline (`self.Spline`))
  (`SceneComponent.K2_SetWorldLocation` (`self.StartMesh`) (`SplineComponent.GetLocationAtSplinePoint` _spline 0 "World") false false)
  (`SceneComponent.K2_SetWorldLocation` (`self.EndMesh`) (`SplineComponent.GetLocationAtSplinePoint` _spline (- (`SplineComponent.GetNumberOfSplinePoints` _spline) 1) "World") false false))

(fn `UserConstructionScript`
  (locals (LoopIndex :type Integer))
  (bind (_returnvalue_x _returnvalue_y) (`KismetMathLibrary.BreakVector` (`self.GetActorScale3D`)))
  (if (`self.AllowScalling?`)
    (set `self.SectionLenght` (* _returnvalue_y 100.0)))
  (if (`self.MustBeFullLenghtMeshes?`)
    (for _index (range (`KismetMathLibrary.FTrunc` (/ (`SplineComponent.GetSplineLength` (`self.Spline`)) (`self.SectionLenght`))))
      (set `local.LoopIndex` _index)
      (bind _returnvalue (`AddComponent|NODE_AddSplineMeshComponent-0` :!label _label))
      (`StaticMeshComponent.SetStaticMesh` _returnvalue (`self.SplineMesh`))
      (`SplineMeshComponent.SetForwardAxis` _returnvalue "Y" true)
      (bind (_position _tangent) (`self.get_Start_Pos /Tangent` (`local.LoopIndex`)))
      (bind (_position_2 _tangent_2) (`self.Get_End_Pos/Tangent` (`local.LoopIndex`)))
      (`SplineMeshComponent.SetStartAndEnd` _returnvalue _position _tangent _position_2 _tangent_2 true)
      (`PrimitiveComponent.SetCollisionEnabled` _returnvalue (`self.CollisionType`))
      (`self.Set_Start_End_Meshes`))
    (else
      (for _index_2 (range (+ (`KismetMathLibrary.FTrunc` (/ (`SplineComponent.GetSplineLength` (`self.Spline`)) (`self.SectionLenght`))) 1))
        (set `local.LoopIndex` _index_2)
        (goto _label)))))