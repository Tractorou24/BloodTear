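; Test Blueprint for an enemy life bar, drawn on a plane with a dynamic instance of M_EnemyLifeBar.
; Each player pawn overlap with the box lowers Life and updates the material's life percentage immediately.
; A retriggerable delay waits for hits to stop, then a self-calling event with short delays steps a trailing damage value down to Life, halting if hit again.
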(event `self.ReceiveBeginPlay`
  ;[0 0 0] ConditionActivation
  (add `PrimitiveComponent.OnComponentBeginOverlap` (`self.Box`) (delegate `TakingHit`))
  ;[0 0 0] LifeBarMaterialSet
  (bind _returnvalue (`KismetMaterialLibrary.CreateDynamicMaterialInstance` "/Game/Art/Materials/ComplexMaterials/M_EnemyLifeBar.M_EnemyLifeBar"))
  (bind _output_get (set `self.DynamicMaterial` _returnvalue))
  (`PrimitiveComponent.SetMaterial` (`self.Plane`) 0 _output_get))

(event `TakingHit`
  (params (OverlappedComponent :type "PrimitiveComponent Object Reference") (OtherActor :type "Actor Object Reference") (OtherComp :type "PrimitiveComponent Object Reference") (OtherBodyIndex :type Integer) (bFromSweep :type Boolean) (SweepResult :type "HitResult Structure (by ref)"))
  ;[0 0 0] ConditionActivation
  (if (== OtherActor (`GameplayStatics.GetPlayerPawn` 0))
    ;[0 0 0] LifeBarAnimationWithMaterial
    (bind _output_get (set `self.Life` (- (`self.Life`) 0.05)))
    (`MaterialInstanceDynamic.SetScalarParameterValue` (`self.DynamicMaterial`) "PercentageLife" _output_get)
    (set `self.TakingHits` true)
    (`KismetSystemLibrary.RetriggerableDelay` (`self.DelayTime`))
    (set `self.TakingHits` false)
    (`self.DelayLife`)))

(event `DelayLife`
  ;[0 0 0] LifeBarAnimationWithMaterial
  (if (not (< (`self.OldLife`) (`self.Life`)))
    (bind _output_get (set `self.OldLife` (- (`self.OldLife`) 0.01)))
    (`MaterialInstanceDynamic.SetScalarParameterValue` (`self.DynamicMaterial`) "PercentageLifeWithDelay" _output_get)
    (`KismetSystemLibrary.Delay` 0.01)
    (if (not (`self.TakingHits`))
      (`self.DelayLife`))))

(fn `UserConstructionScript`)