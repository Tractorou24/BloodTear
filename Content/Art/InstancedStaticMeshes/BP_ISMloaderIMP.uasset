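; Actor that fills an instanced static mesh component, Imp, from transforms stored in the Data_IMP data table.
; The construction script loops by index over the row count and looks up rows named by that number.
; Each found row becomes a component-space instance from its translation, quaternion rotation (converted to a rotator) and scale.
; The event graph holds only disabled stubs, so there is no runtime logic.
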(fn `UserConstructionScript`
  (bind _outrownames (`DataTableFunctionLibrary.GetDataTableRowNames` "/Game/Art/InstancedStaticMeshes/data_IMP.data_IMP"))
  (for _index (range (+ (`KismetArrayLibrary.Array_Length` _outrownames) 1))
    (bind _returnvalue (`|GetDataTableRow` "/Game/Art/InstancedStaticMeshes/data_IMP.data_IMP" (`KismetStringLibrary.Conv_StringToName` (`KismetStringLibrary.Conv_IntToString` _index)))
      (:`then`
        (bind (_id _tx _ty _tz _rw _rx _ry _rz _sx _sy _sz) (break `/Game/Art/InstancedStaticMeshes/F_ISMimport_01` _returnvalue))
        (`InstancedStaticMeshComponent.AddInstance` (`self.imp`) (`KismetMathLibrary.MakeTransform` (`KismetMathLibrary.MakeVector` _tx _ty _tz) (`KismetMathLibrary.MakeRotator` (.roll (`KismetMathLibrary.Quat_Rotator` (`KismetMathLibrary.MakeQuat` _rx _ry _rz _rw))) (.pitch (`KismetMathLibrary.Quat_Rotator` (`KismetMathLibrary.MakeQuat` _rx _ry _rz _rw))) (.yaw (`KismetMathLibrary.Quat_Rotator` (`KismetMathLibrary.MakeQuat` _rx _ry _rz _rw)))) (`KismetMathLibrary.MakeVector` _sx _sy _sz)) false)))))