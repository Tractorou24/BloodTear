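; Imp enemy character that grants jump and base attack abilities, seeds its AI blackboard, plays an FMOD spawn sound and shows hit/hover material feedback.
; After a wind-up and line-of-sight check, Tick drives the leap along a custom-gravity arc until a trace hits.
; Tick also circles the target, reversing when blocked and retreating when too close.
; Loose gameplay tags signal movement states; death while attacking decrements the blackboard attacker count.
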(event `self.ReceiveBeginPlay`
  (bind _returnvalue (`AIBlueprintHelperLibrary.GetBlackboard` null))
  (bind _mesh (`self.Mesh`))
  (bind _abilitysystemcomponent (`self.AbilitySystemComponent`))
  (`|ExecutionSequence`
    (:`then_0`
      (bind _returnvalue_2 (`AbilitySystemComponent.K2_GiveAbility` _abilitysystemcomponent "/Game/Characters/Imp/BPGA_ImpJump.BPGA_ImpJump_C" 0 -1))
      (bind _asbpga_imp_jump (cast `/Game/Characters/Imp/BPGA_ImpJump` (`.ReturnValue` (`AbilitySystemBlueprintLibrary.GetGameplayAbilityFromSpecHandle` _abilitysystemcomponent _returnvalue_2))))
      (set `/Game/Characters/Imp/BPGA_ImpJump.Damages` (`self.AttackDamage`) _asbpga_imp_jump)
      (bind _returnvalue_3 (`AbilitySystemComponent.K2_GiveAbility` _abilitysystemcomponent "/Game/Characters/Imp/BPGA_ImpBaseAttack.BPGA_ImpBaseAttack_C" 0 -1))
      (bind _asbpga_imp_base_attack (cast `/Game/Characters/Imp/BPGA_ImpBaseAttack` (`.ReturnValue` (`AbilitySystemBlueprintLibrary.GetGameplayAbilityFromSpecHandle` _abilitysystemcomponent _returnvalue_3))))
      (set `/Game/Characters/Imp/BPGA_ImpBaseAttack.Damages` (`self.AttackSecondaryDamage`) _asbpga_imp_base_attack)
      (`BlackboardComponent.SetValueAsFloat` _returnvalue "DetectionRange" (`self.DetectionRange`))
      (`BlackboardComponent.SetValueAsFloat` _returnvalue "AttackRange" (`self.AttackRange`))
      (`BlackboardComponent.SetValueAsFloat` _returnvalue "AttackSecondaryRange" (`self.AttackSecondaryRange`))
      (`BlackboardComponent.SetValueAsFloat` _returnvalue "WaitAfterMoveTime" (`self.WaitAfterMoveTime`))
      (`BlackboardComponent.SetValueAsFloat` _returnvalue "MaxAttackRange" (`self.MaxAttackRange`))
      (`BlackboardComponent.SetValueAsFloat` _returnvalue "AttackDelay" (`self.AttackDelay`))
      (`BlackboardComponent.SetValueAsInt` _returnvalue "MaxAttacking" (`self.MaxAttacking`)))
    (:`then_1`
      ;[0 0 0] Setup FeedBack Materials
      (bind _returnvalue_4 (`KismetMaterialLibrary.CreateDynamicMaterialInstance` "/Game/Art/Materials/MasterMaterials/Outline/MM_Outline.MM_Outline"))
      (set `self.DynamicOverlayMaterial` _returnvalue_4)
      (for (_array_element _array_index) (`MeshComponent.GetMaterials` _mesh)
        (bind _returnvalue_5 (`KismetMaterialLibrary.CreateDynamicMaterialInstance` _array_element))
        (`KismetArrayLibrary.Array_Add` (`self.DynamicMaterial`) _returnvalue_5)
        (`PrimitiveComponent.SetMaterial` _mesh _array_index _returnvalue_5)))
    (:`then_2`
      ;[0 0 0] Feedback Hit
      (add `self.OnHitDelegate` (delegate `OnHitDelegate_Event`)))
    (:`then_3`
      ;[0.3633 0 0.5104] FMOD - Imp Spawn
      (`FMODBlueprintStatics.PlayEvent2D` "/Game/FMOD/Events/SFX/Characters/Diablotin/Diablotin_Spawn.Diablotin_Spawn"))))

(event `OnHitDelegate_Event` :!signature `self.OnHitDelegate`
  (params (DamageAmount :type "Float (single-precision)"))
  ;[0 0 0] Feedback Hit
  (bind (_direction _newtrack_0) (`Timeline|Timeline` :!via `PlayFromStart`)
    (:`Update`
      (`MaterialInstanceDynamic.SetScalarParameterValue` (`self.DynamicMaterial`) "HitIntensity" _newtrack_0))))

(event `self.MouseInteractableComponent.OnMouseHoverStart`
  ;[0 0 0] Feedback Outline
  (`MeshComponent.SetOverlayMaterial` (`self.Mesh`) (`self.DynamicOverlayMaterial`)))

(event `self.MouseInteractableComponent.OnMouseHoverEnd`
  ;[0 0 0] Feedback Outline
  (`MeshComponent.SetOverlayMaterial` (`self.Mesh`) null))

(event `self.ReceiveTick`
  (params (DeltaSeconds :type "Float (single-precision)"))
  (`SceneComponent.K2_SetWorldRotation` (`self.UIEnemyInfoComponent`) (struct :`Pitch` 45.0 :`Yaw` 135.0) false false)
  (if (`self.IsJumping`)
    (`self.Jumping` DeltaSeconds)
    (elif (`self.IsMovingAroundTarget`)
      (`self.MovingAroundTarget` DeltaSeconds))))

(event `Attack`
  (bind (_returnvalue_roll _returnvalue_pitch _returnvalue_yaw) (`KismetMathLibrary.BreakRotator` (`self.K2_GetActorRotation`)))
  (bind _returnvalue (`self.K2_GetActorLocation`))
  (bind _asynctaskproxy (`GameplayTask_WaitDelay.TaskWaitDelay` (`AIBlueprintHelperLibrary.GetAIController` self) (`self.WaitPrepareJumpTime`))
    (:`then`
      (set `self.PreparingJumpAsyncTask` _asynctaskproxy))
    (:`OnFinish`
      (if (`/Game/Art/Anims/Diablotin/ABP/ABP_Diablotin_01.Is Preparing Jump` (`self.ABP`))
        (set `/Game/Art/Anims/Diablotin/ABP/ABP_Diablotin_01.Is Preparing Jump` false (`self.ABP`))
        (`BlackboardComponent.SetValueAsBool` (`AIBlueprintHelperLibrary.GetBlackboard` null) "IsPreparingJump" false)
        (bind _asactor (cast `Actor` (`BlackboardComponent.GetValueAsObject` (`AIBlueprintHelperLibrary.GetBlackboard` null) "Target")))
        (bind _returnvalue_2 (`self.K2_GetActorLocation` _asactor))
        (bind _outhit (`KismetSystemLibrary.LineTraceSingle` _returnvalue_2 (`self.K2_GetActorLocation`) "TraceTypeQuery1" false (`|MakeArray` self :!type "Actor Object Reference") "ForDuration" true (struct :`R` 1.0 :`A` 1.0) (struct :`G` 1.0 :`A` 1.0) 1.0))
        (if (not (`GameplayStatics.BreakHitResult` _outhit))
          (set `/Game/Art/Anims/Diablotin/ABP/ABP_Diablotin_01.Is Jumping` true (`self.ABP`))
          (set `self.IsJumping` true)
          (`AbilitySystemBlueprintLibrary.AddLooseGameplayTags` self (`BlueprintGameplayTagLibrary.MakeLiteralGameplayTagContainer` (struct :`GameplayTags` (struct :`(TagName` "Ability.ImpJump.Jumping")))))
          (set `self.StartLocation` _returnvalue)
          (bind _returnvalue_3 (`MathAI.GetProjectileCustomGravity` (`self.JumpAngle`) (`self.JumpSpeed`) (`KismetMathLibrary.Vector_Distance2D` _returnvalue_2 _returnvalue)))
          (set `self.JumpGravity` _returnvalue_3)
          (set `self.JumpDuration` (/ (* (* (`self.JumpSpeed`) 2.0) (`KismetMathLibrary.DegSin` (`self.JumpAngle`))) (`self.JumpGravity`)))
          (bind _output_get (set `self.StartRotationYaw` _returnvalue_yaw))
          (set `self.LastFlyControlDelta` _output_get)
          (`PrimitiveComponent.SetEnableGravity` (`self.CapsuleComponent`) false)
          (`Controller.StopMovement` (`self.GetController`))
          (else
            (`AbilitySystemBlueprintLibrary.AddLooseGameplayTags` self (`BlueprintGameplayTagLibrary.MakeLiteralGameplayTagContainer` (struct :`GameplayTags` (struct :`(TagName` "Ability.ImpJump.Canceled")))))))))))

(event `MovingAroundTarget`
  (params (DeltaTime :type "Float (double-precision)"))
  (bind _returnvalue (`self.K2_GetActorLocation`))
  (bind _returnvalue_2 (`self.K2_GetActorLocation`))
  (bind _movingaroundasynctask (`self.MovingAroundAsyncTask`))
  (bind _movearoundtargetminimalradius (`self.MoveAroundTargetMinimalRadius`))
  (bind _returnvalue_3 (`AIBlueprintHelperLibrary.GetAIController` self))
  (`|ExecutionSequence`
    (:`then_0`
      (`/Engine/EditorBlueprintResources/StandardMacros.DoOnce` false :!label _label
        (:`Completed`
          (bind _asynctaskproxy (`GameplayTask_WaitDelay.TaskWaitDelay` _returnvalue_3 (`self.MoveAroundDuration`))
            (:`then`
              (set `self.MovingAroundAsyncTask` _asynctaskproxy))
            (:`OnFinish`
              (`Controller.StopMovement` _returnvalue_3)
              (`AbilitySystemBlueprintLibrary.AddLooseGameplayTags` self (`BlueprintGameplayTagLibrary.MakeLiteralGameplayTagContainer` (struct :`GameplayTags` (struct :`(TagName` "Ability.ImpMoveAroundTarget.Stop")))))
              (goto _label :!via `Reset`))))))
    (:`then_1`
      (bind _asactor (cast `Actor` (`BlackboardComponent.GetValueAsObject` (`AIBlueprintHelperLibrary.GetBlackboard` null) "Target")))
      (bind _returnvalue_4 (`self.K2_GetActorLocation` _asactor))
      (bind _returnvalue_5 (`KismetMathLibrary.Vector_Distance` _returnvalue_4 _returnvalue_2))
      (if (>= _returnvalue_5 _movearoundtargetminimalradius)
        (if (not (`self.IsRepositioning`))
          (bind _result (`MathAI.GetNextPointOnCircleByAngle` _returnvalue_4 _returnvalue (`self.MoveAroundTargetSpeed`) DeltaTime (`self.MoveAroundTargetClockwise`)))
          (bind _returnvalue_6 (+ _result (* (`self.GetActorForwardVector`) 50.0)))
          (bind (_outhit _returnvalue_7) (`KismetSystemLibrary.SphereTraceSingle` _returnvalue_6 _returnvalue_6 20.0 "TraceTypeQuery1"))
          (if (and (not _returnvalue_7) (`AIBlueprintHelperLibrary.IsValidAILocation` _returnvalue_6))
            (if (`AIBlueprintHelperLibrary.IsValidAILocation` _result)
              (`self.K2_SetActorRotation` (`KismetMathLibrary.RLerp` (`self.K2_GetActorRotation`) (`KismetMathLibrary.FindLookAtRotation` _returnvalue _result) 1.0))
              (`self.K2_SetActorLocation` _result)
              (`KismetSystemLibrary.DrawDebugBox` _result (5.0 5.0 5.0) (struct :`R` 1.0 :`G` 0.078394 :`A` 1.0) (struct) 1.0))
            (else
              (set `self.MoveAroundTargetClockwise` (not (`self.MoveAroundTargetClockwise`))))))
        (else
          (`|DoOnceMultiInput` :!label _label_2
            (:`A Out`
              (set `self.IsRepositioning` true)
              (bind _returnvalue_8 (+ _returnvalue_2 (* (* (- _movearoundtargetminimalradius _returnvalue_5) 1.3) (`self.GetActorForwardVector`) -1.0)))
              (`|AIMoveTo` self _returnvalue_8 null
                (:`then`
                  (`KismetSystemLibrary.DrawDebugBox` _returnvalue_8 (5.0 5.0 5.0) (struct :`R` 1.0 :`G` 0.078394 :`A` 1.0) (struct) 1.0))
                (:`OnSuccess`
                  (if (`KismetSystemLibrary.IsValid` _movingaroundasynctask) :!label _label_3
                    (`GameplayTask.EndTask` _movingaroundasynctask)
                    (`Controller.StopMovement` (`AIBlueprintHelperLibrary.GetAIController` self))
                    (`AbilitySystemBlueprintLibrary.AddLooseGameplayTags` self (`BlueprintGameplayTagLibrary.MakeLiteralGameplayTagContainer` (struct :`GameplayTags` (struct :`(TagName` "Ability.ImpMoveAroundTarget.Stop")))))
                    (goto _label_2 :!via `Reset In`)
                    (else
                      (goto _label_2 :!via `Reset In`))))
                (:`OnFail`
                  (goto _label_3))))
            (:`Reset Out`
              (set `self.IsRepositioning` false)
              (goto _label :!via `Reset`))))))))

(event `self.OnDeath_Blueprint`
  (bind _returnvalue (`AIBlueprintHelperLibrary.GetBlackboard` null))
  (if (`BlackboardComponent.GetValueAsBool` _returnvalue "IsAttacking")
    (bind _result (`/Engine/EditorBlueprintResources/StandardMacros.DecrementInt` (`BlackboardComponent.GetValueAsInt` _returnvalue "CurrentAttacking"))
      (:`  `
        (`BlackboardComponent.SetValueAsInt` _returnvalue "CurrentAttacking" _result)))))

(fn `CancelJump`
  (bind _preparingjumpasynctask (`self.PreparingJumpAsyncTask`))
  (if (`KismetSystemLibrary.IsValid` _preparingjumpasynctask)
    (`GameplayTask.EndTask` _preparingjumpasynctask)
    (set `/Game/Art/Anims/Diablotin/ABP/ABP_Diablotin_01.Is Preparing Jump` false (`self.ABP`))
    (`AbilitySystemBlueprintLibrary.AddLooseGameplayTags` self (`BlueprintGameplayTagLibrary.MakeLiteralGameplayTagContainer` (struct :`GameplayTags` (struct :`(TagName` "Ability.ImpJump.Canceled")))))
    (`BlackboardComponent.SetValueAsBool` (`AIBlueprintHelperLibrary.GetBlackboard` null) "IsPreparingJump" false)))

(fn `Jumping`
  (params (DeltaTime :type "Float (double-precision)"))
  (bind _output_get (set `self.JumpTimeAccumulator` (+ DeltaTime (`self.JumpTimeAccumulator`))))
  (bind _result (`MathAI.GetProjectilePositionByTime` _output_get (`self.JumpAngle`) (`self.StartRotationYaw`) (`self.JumpSpeed`) (`self.JumpGravity`)))
  (bind _returnvalue (+ _result (`self.StartLocation`)))
  (bind (_outhit _returnvalue_2) (`KismetSystemLibrary.LineTraceSingle` (`self.K2_GetActorLocation`) (- (+ _returnvalue (* (`self.GetActorForwardVector`) 30.0)) (0.0 0.0 30.0)) "TraceTypeQuery1"))
  (if _returnvalue_2
    (set `self.IsJumping` false)
    (`PrimitiveComponent.SetEnableGravity` (`self.CapsuleComponent`) true)
    (set `self.JumpTimeAccumulator` 0.0)
    (`AbilitySystemBlueprintLibrary.AddLooseGameplayTags` self (`BlueprintGameplayTagLibrary.MakeLiteralGameplayTagContainer` (struct :`GameplayTags` (struct :`(TagName` "Ability.ImpJump.Landing")))))
    (else
      (`self.K2_SetActorLocation` _returnvalue)))
  (if (<= (- (`self.JumpDuration`) 0.15) (`self.JumpTimeAccumulator`))
    (set `/Game/Art/Anims/Diablotin/ABP/ABP_Diablotin_01.Is Jumping` false (`self.ABP`))))

(fn `PrepareJump`
  (set `/Game/Art/Anims/Diablotin/ABP/ABP_Diablotin_01.Is Preparing Jump` true (`self.ABP`))
  (`BlackboardComponent.SetValueAsBool` (`AIBlueprintHelperLibrary.GetBlackboard` null) "IsPreparingJump" true))

(fn `StartMovingAroundTarget`
  (set `self.IsMovingAroundTarget` true)
  (set `self.MoveAroundTargetClockwise` (== (`KismetMathLibrary.RandomInteger` 2) 0)))

(fn `StopMovingAroundTarget`
  (set `self.IsMovingAroundTarget` false))

(fn `UserConstructionScript`)