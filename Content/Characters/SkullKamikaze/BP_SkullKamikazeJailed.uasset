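; BP_SkullKamikazeJailed is a skull kamikaze enemy that attacks by exploding.
; On BeginPlay it copies detection, trigger range and speed tuning into the Blackboard, then grants BPGA_SkullKamikazeExplosion and injects delay, damage and radius into the ability instance.
; It also creates dynamic mesh and outline materials, storing the outline without applying it here.
; Helpers start or destroy the Canalisation component, while StartExplosion activates the Explosion component and destroys the actor shortly after.
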(event `self.ReceiveBeginPlay`
  (bind _mesh (`self.Mesh`))
  (bind _abilitysystemcomponent (`self.AbilitySystemComponent`))
  (`|ExecutionSequence`
    (:`then_0`
      (`BlackboardComponent.SetValueAsFloat` (`AIBlueprintHelperLibrary.GetBlackboard` null) "DetectionRange" (`self.DetectionRange`))
      (`BlackboardComponent.SetValueAsFloat` (`AIBlueprintHelperLibrary.GetBlackboard` null) "ExplosionTriggerRange" (`self.ExplosionTriggerRange`))
      (`BlackboardComponent.SetValueAsFloat` (`AIBlueprintHelperLibrary.GetBlackboard` null) "AttackMoveSpeed" (`self.AttackMoveSpeed`))
      (bind _returnvalue (`AbilitySystemComponent.K2_GiveAbility` _abilitysystemcomponent "/Game/Characters/SkullKamikaze/BPGA_SkullKamikazeExplosion.BPGA_SkullKamikazeExplosion_C" 0 -1))
      (bind _asbpga_skull_kamikaze_explosion (cast `/Game/Characters/SkullKamikaze/BPGA_SkullKamikazeExplosion` (`.ReturnValue` (`AbilitySystemBlueprintLibrary.GetGameplayAbilityFromSpecHandle` _abilitysystemcomponent _returnvalue))))
      (set `/Game/Characters/SkullKamikaze/BPGA_SkullKamikazeExplosion.ExplosionDelay` (`self.ExplosionDelay`) _asbpga_skull_kamikaze_explosion)
      (set `/Game/Characters/SkullKamikaze/BPGA_SkullKamikazeExplosion.Damages` (`self.ExplosionDamages`) _asbpga_skull_kamikaze_explosion)
      (set `/Game/Characters/SkullKamikaze/BPGA_SkullKamikazeExplosion.ExplosionRadius` (`self.ExplosionRadius`) _asbpga_skull_kamikaze_explosion))
    (:`then_1`
      (bind _returnvalue_2 (`KismetMaterialLibrary.CreateDynamicMaterialInstance` "/Game/Art/Materials/MasterMaterials/Outline/MM_Outline.MM_Outline"))
      (set `self.DynamicOverlayMaterial` _returnvalue_2)
      (bind _returnvalue_3 (`KismetMaterialLibrary.CreateDynamicMaterialInstance` (`PrimitiveComponent.GetMaterial` _mesh 0)))
      (bind _output_get (set `self.DynamicMaterial` _returnvalue_3))
      (`PrimitiveComponent.SetMaterial` _mesh 0 _output_get))))

(event `StartExplosion`
  (`ActorComponent.Activate` (`self.Explosion`) false)
  (`KismetSystemLibrary.Delay` 0.5)
  (`self.K2_DestroyActor`))

(fn `StartCanalisation`
  (`ActorComponent.Activate` (`self.Canalisation`) false))

(fn `StopCanalisation`
  (`ActorComponent.K2_DestroyComponent` (`self.Canalisation`)))

(fn `UserConstructionScript`)