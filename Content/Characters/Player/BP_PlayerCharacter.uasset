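; Player character Blueprint that links the player camera, Gameplay Ability System and weapon inventory.
; BeginPlay grants dash, base attack and potion abilities and binds hit, potion and level-up feedback, with level-ups also adding potions.
; Weapon swaps reapply max speed through a set-by-caller effect.
; Dynamic materials flash on hits, Tick aims an arrow at the cursor, and helpers lock movement with optional invulnerability.
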(event `self.ReceiveBeginPlay`
  (bind _abilitysystemcomponent (`self.AbilitySystemComponent`))
  (`|ExecutionSequence`
    (:`then_0`
      (bind _returnvalue (`GameplayStatics.GetActorOfClass` "/Game/Characters/Player/BP_PlayerCamera.BP_PlayerCamera_C"))
      (set `/Game/Characters/Player/BP_PlayerCamera.PlayerRef` self _returnvalue)
      (bind _asens_player_controller (cast `EnsPlayerController` (`self.GetController`)))
      (`PlayerController.SetViewTargetWithBlend` _asens_player_controller _returnvalue 0.0 "VTBlend_Linear" 0.0 false)
      (add `Inventory.OnSwapWeapon` (`self.Inventory`) (delegate `OnWeaponChange`))
      (bind _returnvalue_2 (`AbilitySystemComponent.K2_GiveAbility` _abilitysystemcomponent "/Game/Characters/Player/Abilities/BPGA_Dash.BPGA_Dash_C" 0 -1))
      (bind _asbpga_dash (cast `/Game/Characters/Player/Abilities/BPGA_Dash` (`.ReturnValue` (`AbilitySystemBlueprintLibrary.GetGameplayAbilityFromSpecHandle` _abilitysystemcomponent _returnvalue_2))))
      (set `EnsGameplayAbilityBase.CooldownDuration` (`self.Cooldown Duration`) _asbpga_dash)
      (`EnsAbilitySystemComponent.SetInputBinding` (`self.AbilitySystemComponent`) "/Game/Inputs/Actions/IA_Dash.IA_Dash" _returnvalue_2)
      (`AbilitySystemComponent.K2_GiveAbility` (`self.AbilitySystemComponent`) "/Game/Characters/Player/Abilities/BPGA_BaseAttack.BPGA_BaseAttack_C" 0 -1)
      (bind _returnvalue_3 (`AbilitySystemComponent.K2_GiveAbility` (`self.AbilitySystemComponent`) "/Game/Characters/Player/Abilities/BPGA_Potion.BPGA_Potion_C" 0 -1))
      (`EnsAbilitySystemComponent.SetInputBinding` (`self.AbilitySystemComponent`) "/Game/Inputs/Actions/IA_Potion.IA_Potion" _returnvalue_3))
    (:`then_1`
      ;[0 0 0] Setup Materials For Feedback
      (for (_array_element _array_index) (`MeshComponent.GetMaterials` (`self.Mesh`))
        (bind _returnvalue_4 (`KismetMaterialLibrary.CreateDynamicMaterialInstance` _array_element))
        (`KismetArrayLibrary.Array_Add` (`self.DynamicMaterials`) _returnvalue_4)
        (`PrimitiveComponent.SetMaterial` (`self.Mesh`) _array_index _returnvalue_4)))
    (:`then_2`
      ;[0 0 0] Feedback Hit
      (add `self.OnHitDelegate` (delegate `TakingDamage`)))
    (:`then_3`
      (bind _returnvalue_5 (`Inventory.GetCurrentWeapon` (`self.Inventory`)))
      (`self.ApplySpeedModifier` _returnvalue_5))
    (:`then_4`
      (bind _returnvalue_6 (`AbilitySystemComponent.GetAttributeSet` (`self.AbilitySystemComponent`) "/Script/ENS.EnsPotionAttributeSet"))
      (bind _asens_potion_attribute_set (cast `EnsPotionAttributeSet` _returnvalue_6))
      (add `EnsPotionAttributeSet.OnHealthPotionUsed` _asens_potion_attribute_set (delegate `OnPotionUsed`)))
    (:`then_5`
      (add `self.OnLevelUp` (delegate `FX`))
      (add `self.OnLevelUp` (delegate `AddPotion`)))))

(event `OnWeaponChange`
  (params (NewWeapon :type "BaseWeapon Object Reference"))
  (set `self.CurrentWeaponSet` (cast `/Game/BP/AnimBP/E_WeaponSets` (`KismetMathLibrary.Conv_IntToByte` (`KismetArrayLibrary.Array_Find` (`Inventory.Weapons` (`self.Inventory`)) (`GameplayStatics.GetObjectClass` NewWeapon)))))
  (`AbilitySystemComponent.RemoveActiveEffectsWithAppliedTags` (`self.AbilitySystemComponent`) (struct :`GameplayTags` (struct :`(TagName` "Ability.MaxSpeed"))))
  (`self.ApplySpeedModifier` NewWeapon))

(event `TakingDamage` :!signature `self.OnHitDelegate`
  (params (DamageAmount :type "Float (single-precision)"))
  ;[0 0 0] Feedback Hit
  (`|ExecutionSequence`
    (:`then_0`
      (bind (_direction _newtrack_0) (`Timeline|Timeline` :!via `PlayFromStart`)
        (:`Update`
          (`MaterialInstanceDynamic.SetScalarParameterValue` (`self.DynamicMaterials`) "HitIntensity" _newtrack_0))))
    (:`then_1`
      (`NiagaraFunctionLibrary.SpawnSystemAtLocation` "/Game/Art/FX/Hit_Effect/NS_HIT_IMP_01.NS_HIT_IMP_01" (`self.K2_GetActorLocation`)))))

(event `OnPotionUsed`
  (params (Remaining :type Integer))
  (`|PlayMontage` (`self.Mesh`) "/Game/Art/TempAsset/AnimsImports/HeavySet/AM_MainCharacter_DrinkingPotionHeavy_01.AM_MainCharacter_DrinkingPotionHeavy_01" 1.0 0.0 "Spine_1"))

(event `FX` :!signature `self.OnLevelUp`
  (params (NewLevel :type Integer64))
  (`NiagaraFunctionLibrary.SpawnSystemAtLocation` "/Game/Art/FX/Level_Up/NS_Level_Up.NS_Level_Up" (`self.K2_GetActorLocation`)))

(event `AddPotion` :!signature `self.OnLevelUp`
  (params (NewLevel :type Integer64))
  (bind _abilitysystemcomponent (`self.AbilitySystemComponent`))
  (`AbilitySystemComponent.BP_ApplyGameplayEffectSpecToSelf` _abilitysystemcomponent (`AbilitySystemComponent.MakeOutgoingSpec` _abilitysystemcomponent "/Game/Characters/Player/Abilities/BPGE_AddPotion.BPGE_AddPotion_C" 1.0 (`AbilitySystemComponent.MakeEffectContext` _abilitysystemcomponent))))

(event `self.ReceiveTick`
  (params (DeltaSeconds :type "Float (single-precision)"))
  (bind _pivotpointfeedbackarrow (`self.PivotPointFeedBackArrow`))
  (bind _hitresult (`self.GetHitResultUnderCursor` "TraceTypeQuery3"))
  (if (`GameplayStatics.BreakHitResult` _hitresult)
    (bind (_returnvalue_roll _returnvalue_pitch _returnvalue_yaw) (`KismetMathLibrary.BreakRotator` (`KismetMathLibrary.FindLookAtRotation` (`SceneComponent.K2_GetComponentLocation` _pivotpointfeedbackarrow) (`.Location` (`GameplayStatics.BreakHitResult` _hitresult)))))
    (`SceneComponent.K2_SetWorldRotation` _pivotpointfeedbackarrow (`KismetMathLibrary.MakeRotator` 0.0 0.0 _returnvalue_yaw) false false)))

(event `self.OnBaseAttack`
  (bind _returnvalue (`Inventory.GetCurrentWeapon` (`self.Inventory`)))
  (bind _returnvalue_2 (`BaseWeapon.GetCurrentCameraShake` _returnvalue))
  (if (`KismetSystemLibrary.IsValidClass` _returnvalue_2)
    (`CameraShakeSourceComponent.StartCameraShake` :`self` (`self.CameraShakeSource`) :`InCameraShake` _returnvalue_2)))

(fn `ApplySpeedModifier`
  (params (Weapon :type "BaseWeapon Object Reference"))
  (bind _abilitysystemcomponent (`self.AbilitySystemComponent`))
  (bind _returnvalue (`AbilitySystemBlueprintLibrary.AssignTagSetByCallerMagnitude` (`AbilitySystemComponent.MakeOutgoingSpec` _abilitysystemcomponent "/Game/Characters/Player/Abilities/BPGE_SpeedModifier.BPGE_SpeedModifier_C" 0.0 (`AbilitySystemComponent.MakeEffectContext` _abilitysystemcomponent)) (struct :`TagName` "Ability.MaxSpeed") (`BaseWeapon.PlayerMaxSpeed` Weapon)))
  (`AbilitySystemComponent.BP_ApplyGameplayEffectSpecToSelf` (`self.AbilitySystemComponent`) _returnvalue))

(fn `Block Movements`
  (params (IsVulnerable :type Boolean))
  (bind _charactermovement (`self.CharacterMovement`))
  (if (not IsVulnerable)
    (`AbilitySystemBlueprintLibrary.AddLooseGameplayTags` self (`BlueprintGameplayTagLibrary.MakeLiteralGameplayTagContainer` (struct :`GameplayTags` (struct :`(TagName` "Ability.Invulnerable"))))))
  (`MovementComponent.StopMovementImmediately` _charactermovement)
  (`CharacterMovementComponent.SetMovementMode` _charactermovement "MOVE_None" 0)
  (`AnimInstance.SetRootMotionMode` (`SkeletalMeshComponent.GetAnimInstance` (`self.GetComponentByClass` "/Script/Engine.SkeletalMeshComponent")) "IgnoreRootMotion"))

(fn `FXPotion`
  (`NiagaraFunctionLibrary.SpawnSystemAttached` "/Game/Art/FX/Heal/NS_Heal_02.NS_Heal_02" (`self.CapsuleComponent`) "None" (0.0 0.0 10.0) (struct) "KeepRelativeOffset"))

(fn `GetHitResultUnderCursor`
  (params (Channel :type "ETraceTypeQuery Enum" :default "TraceTypeQuery1"))
  (returns (HitResult :type "HitResult Structure"))
  (bind _asplayer_controller (cast `PlayerController` (`self.GetController`)))
  (bind (_hitresult _returnvalue) (`PlayerController.GetHitResultUnderCursorByChannel` _asplayer_controller Channel true))
  (if _returnvalue
    (return _hitresult)))

(fn `UnBlockMovements`
  (`CharacterMovementComponent.SetMovementMode` (`self.CharacterMovement`) "MOVE_Walking" 0)
  (`AnimInstance.SetRootMotionMode` (`SkeletalMeshComponent.GetAnimInstance` (`self.GetComponentByClass` "/Script/Engine.SkeletalMeshComponent")) "RootMotionFromEverything")
  (`AbilitySystemBlueprintLibrary.RemoveLooseGameplayTags` self (`BlueprintGameplayTagLibrary.MakeLiteralGameplayTagContainer` (struct :`GameplayTags` (struct :`(TagName` "Ability.Invulnerable"))))))

(fn `UserConstructionScript`)