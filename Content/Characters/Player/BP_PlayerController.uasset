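; Player controller that manages the player's HUD, lives display, death screen, pause menu and attack facing.
; BeginPlay creates the player info and wave counter widgets, after a delay in distribution builds.
; Losing a life pauses behind a death widget, whose continue event resumes play with timed invulnerability via a loose gameplay tag.
; Tick interpolates the pawn's yaw toward an externally set DesiredRotation while the character attacks and can follow the mouse.
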(event `self.ReceiveBeginPlay`
  (if (`KismetSystemLibrary.IsPackagedForDistribution`)
    (`KismetSystemLibrary.Delay` 5.2))
  (set `self.Lives` 3)
  (set `self.InteractionRadius` 30.0)
  (bind _returnvalue (`|CreateWidget` "/Game/Widget/WB_PlayerInfo.WB_PlayerInfo_C"))
  (bind _output_get (set `self.Widget` _returnvalue))
  (`UserWidget.AddToViewport` _output_get 0)
  (`/Game/Widget/WB_PlayerInfo.UpdateLives` _output_get (`self.Lives`))
  (bind _returnvalue_2 (`|CreateWidget` "/Game/Widget/WB_WaveCounter.WB_WaveCounter_C"))
  (`UserWidget.AddToViewport` _returnvalue_2 0))

(event `self.LostLife`
  (`/Game/Widget/WB_PlayerInfo.UpdateLives` (`self.Widget`) (`self.Lives`))
  (`GameplayStatics.SetGamePaused` true)
  (bind _returnvalue (`|CreateWidget` "/Game/Widget/WB_Die.WB_Die_C" self))
  (`WidgetBlueprintLibrary.SetInputMode_UIOnlyEx` self _returnvalue)
  (`UserWidget.AddToViewport` _returnvalue 0)
  (add `/Game/Widget/WB_Die.OnContinue` _returnvalue (delegate `OnContinue`)))

(event `OnContinue`
  (`WidgetBlueprintLibrary.SetInputMode_GameAndUIEx` self (stale `self.LostLife` _returnvalue) "DoNotLock" false)
  (`Widget.RemoveFromParent` (stale `self.LostLife` _returnvalue))
  (`GameplayStatics.SetGamePaused` false)
  (`AbilitySystemBlueprintLibrary.AddLooseGameplayTags` (`GameplayStatics.GetPlayerCharacter` 0) (`BlueprintGameplayTagLibrary.MakeGameplayTagContainerFromTag` (struct :`TagName` "Ability.Invulnerable")))
  (`KismetSystemLibrary.K2_SetTimerDelegate` (delegate `OnInvulnerabilityEnd`) 2.0))

(event `self.Restart`
  (`GameplayStatics.OpenLevelBySoftObjectPtr` "/Game/Maps/L_MainMenu.L_MainMenu"))

(event `OnInvulnerabilityEnd`
  (`AbilitySystemBlueprintLibrary.RemoveLooseGameplayTags` (`GameplayStatics.GetPlayerCharacter` 0) (`BlueprintGameplayTagLibrary.MakeGameplayTagContainerFromTag` (struct :`TagName` "Ability.Invulnerable"))))

(event `EnhancedInput|/Game/Inputs/Actions/IA_PauseMenu`
  (params (ActionValue :type Boolean) (ElapsedSeconds :type "Float (double-precision)") (TriggeredSeconds :type "Float (double-precision)") (InputAction :type "InputAction Object Reference" :default "/Game/Inputs/Actions/IA_PauseMenu.IA_PauseMenu"))
  (bind _returnvalue (`GameplayStatics.GetPlayerController` 0))
  (:`Started`
    (if (not (`GameplayStatics.IsGamePaused`))
      (set `self.IsPauseMenuOpened` true)
      (bind _returnvalue_2 (`|CreateWidget` "/Game/Widget/WB_PauseMenu.WB_PauseMenu_C" _returnvalue))
      (bind _output_get (set `self.Pause_Menu_Widget` _returnvalue_2))
      (`UserWidget.AddToViewport` _output_get 0)
      (`WidgetBlueprintLibrary.SetInputMode_GameAndUIEx` _returnvalue null "DoNotLock" false)
      (`GameplayStatics.SetGamePaused` true)
      (else
        (set `self.IsPauseMenuOpened` false)
        (`Widget.RemoveFromParent` (`self.Pause_Menu_Widget`))
        (`GameplayStatics.SetGamePaused` false)))))

(event `self.ReceiveTick`
  (params (DeltaSeconds :type "Float (single-precision)"))
  (bind _returnvalue (`self.K2_GetPawn`))
  (bind (_returnvalue_roll _returnvalue_pitch _returnvalue_yaw) (`KismetMathLibrary.BreakRotator` (`self.K2_GetActorRotation` _returnvalue)))
  (bind _asbp_player_character (cast `/Game/Characters/Player/BP_PlayerCharacter` _returnvalue))
  (if (and (`EnsPlayerCharacter.bIsAttacking` _asbp_player_character) (`/Game/Characters/Player/BP_PlayerCharacter.CanFollowMouse` _asbp_player_character))
    (`self.K2_SetActorRotation` _returnvalue (`KismetMathLibrary.RInterpTo` (`KismetMathLibrary.MakeRotator` _returnvalue_roll _returnvalue_pitch _returnvalue_yaw) (`KismetMathLibrary.MakeRotator` _returnvalue_roll _returnvalue_pitch (`self.DesiredRotation`)) (* DeltaSeconds (`self.RotationSpeed`)) 1.0) false)))

(fn `SetDesiredRotation`
  (params (DesiredRotation :type "Float (double-precision)") (UseStyle :type Boolean))
  (set `self.DesiredRotation` DesiredRotation))

(fn `UserConstructionScript`)