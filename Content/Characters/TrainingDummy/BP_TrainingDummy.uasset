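; BP_TrainingDummy is a training dummy character that flashes when hit and respawns a fresh copy at its starting transform when it dies.
; BeginPlay swaps mesh materials for dynamic instances, creates an outline overlay instance, binds the hit delegate and stores the spawn transform.
; Each hit restarts a timeline that drives the HitIntensity material parameter.
; Tick holds the enemy info UI component at a fixed world rotation.
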(event `self.ReceiveBeginPlay`
  (bind _mesh (`self.Mesh`))
  (`|ExecutionSequence`
    (:`then_0`
      ;[0 0 0] Setup FeedBack Materials
      (bind _returnvalue (`KismetMaterialLibrary.CreateDynamicMaterialInstance` "/Game/Art/Materials/MasterMaterials/Outline/MM_Outline.MM_Outline"))
      (set `self.DynamicOverlayMaterial` _returnvalue)
      (for (_array_element _array_index) (`MeshComponent.GetMaterials` _mesh)
        (bind _returnvalue_2 (`KismetMaterialLibrary.CreateDynamicMaterialInstance` _array_element))
        (`KismetArrayLibrary.Array_Add` (`self.DynamicMaterial`) _returnvalue_2)
        (`PrimitiveComponent.SetMaterial` _mesh _array_index _returnvalue_2)))
    (:`then_1`
      ;[0 0 0] Feedback Hit
      (add `EnsCharacterBase.OnHitDelegate` (delegate `OnHitDelegate_Event`)))
    (:`then_2`
      (set `self.Spawn` (`self.GetTransform`)))))

(event `OnHitDelegate_Event`
  (params (DamageAmount :type "Float (single-precision)"))
  ;[0 0 0] Feedback Hit
  (bind (_direction _newtrack_0) (`Timeline|Timeline` :!via `PlayFromStart`)
    (:`Update`
      (`MaterialInstanceDynamic.SetScalarParameterValue` (`self.DynamicMaterial`) "HitIntensity" _newtrack_0))))

(event `self.ReceiveTick`
  (params (DeltaSeconds :type "Float (single-precision)"))
  (`SceneComponent.K2_SetWorldRotation` (`self.UIEnemyInfoComponent`) (struct :`Pitch` 45.0 :`Yaw` 135.0) false false))

(event `self.OnDeath_Blueprint`
  (`|SpawnActorFromClass` "BP_TrainingDummy_C" (`self.Spawn`) "Undefined" "MultiplyWithRoot" null null))

(fn `UserConstructionScript`)