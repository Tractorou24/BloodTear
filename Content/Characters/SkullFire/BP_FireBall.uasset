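; Enemy fireball projectile that charges during a cast, then flies forward to damage the player.
; Initialize starts the cast, setting the shooter's IsCasting blackboard key and playing a montage, then a timer releases movement and overlap checks.
; Player hits apply a SetByCaller GAS damage effect with hardcoded magnitude, ignoring the Damage variable.
; It self-destructs on non-enemy hits, after a lifetime timer, or whenever its shooter is hit or destroyed.
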(event `Cast`
  (`BlackboardComponent.SetValueAsBool` (`AIBlueprintHelperLibrary.GetBlackboard` (`self.Shooter`)) "IsCasting" true)
  (`KismetSystemLibrary.K2_SetTimerDelegate` (delegate `EndCast`) (`self.CastingTime`))
  (`|PlayMontage` (`self.GetComponentByClass` (`self.Shooter`) "/Script/Engine.SkeletalMeshComponent")
    (:`then`
      (bind _returnvalue (`KismetSystemLibrary.K2_SetTimerDelegate` (delegate `Clear`) 10.0))
      (set `self.TimerHandle` _returnvalue))))

(event `EndCast`
  (bind _shooter (`self.Shooter`))
  (set `self.IsCasting` false)
  (`/Engine/EditorBlueprintResources/StandardMacros.IsValid` _shooter
    (:`Is Valid`
      (`BlackboardComponent.SetValueAsBool` (`AIBlueprintHelperLibrary.GetBlackboard` _shooter) "IsCasting" false)
      (bind _outactors (`KismetSystemLibrary.SphereOverlapActors` (`self.K2_GetActorLocation`) 0.15 (`|MakeArray` "ObjectTypeQuery3" :!type "EObjectTypeQuery Enum")))
      (for _array_element _outactors
        (if (`KismetSystemLibrary.IsValid` self)
          (`self.Spell` _array_element))))
    (:`Is Not Valid`
      (`self.K2_DestroyActor`))))

(event `Clear`
  (`self.K2_DestroyActor`))

(event `self.Sphere.OnComponentBeginOverlap`
  (params (OverlappedComponent :type "PrimitiveComponent Object Reference") (OtherActor :type "Actor Object Reference") (OtherComp :type "PrimitiveComponent Object Reference") (OtherBodyIndex :type Integer) (bFromSweep :type Boolean) (SweepResult :type "HitResult Structure (by ref)"))
  (if (`self.IsCasting`)
    _
    (elif (and (`KismetSystemLibrary.IsValid` self) (`KismetSystemLibrary.IsValid` OtherActor))
      (`self.Spell` OtherActor))))

(event `self.ReceiveTick`
  (params (DeltaSeconds :type "Float (single-precision)"))
  (if (not (`self.IsCasting`))
    (`self.K2_AddActorLocalOffset` (* DeltaSeconds (`KismetMathLibrary.MakeVector` (`self.Speed`))))))

(event `self.ReceiveDestroyed`
  (`KismetSystemLibrary.K2_ClearAndInvalidateTimerHandle` (`self.TimerHandle`)))

(event `Initialize`
  (params (Speed :type "Float (double-precision)") (Damage :type "Float (double-precision)") (CastingTime :type "Float (double-precision)") (Shooter :type "/Game/Characters/SkullFire/BP_SkullFire Object Reference"))
  (set `self.Speed` Speed)
  (set `self.Damage` Damage)
  (set `self.CastingTime` CastingTime)
  (bind _output_get (set `self.Shooter` Shooter))
  (add `EnsEnemyBase.OnEnemyDestroyed` _output_get (delegate `CustomEvent`))
  (add `EnsCharacterBase.OnHitDelegate` (`self.Shooter`) (delegate `CustomEvent_0`))
  (`self.Cast`))

(event `CustomEvent`
  (`self.K2_DestroyActor` :!label _label))

(event `CustomEvent_0`
  (params (DamageAmount :type "Float (single-precision)"))
  (`BlackboardComponent.SetValueAsBool` (`AIBlueprintHelperLibrary.GetBlackboard` (`self.Shooter`)) "IsCasting" false)
  (goto _label))

(fn `Spell`
  (params (HitActor :type "Actor Object Reference"))
  (bind _returnvalue (`AbilitySystemBlueprintLibrary.GetAbilitySystemComponent` HitActor))
  (`/Engine/EditorBlueprintResources/StandardMacros.IsValid` HitActor
    (:`Is Valid`
      (if (or (`self.ActorHasTag` HitActor "Enemy") (`self.ActorHasTag` HitActor "EnemyProjectile"))
        _
        (elif (`self.ActorHasTag` HitActor "Player")
          (bind _returnvalue_2 (`AbilitySystemBlueprintLibrary.AssignTagSetByCallerMagnitude` (`AbilitySystemComponent.MakeOutgoingSpec` _returnvalue "/Game/Characters/Player/Abilities/DevelopperTests/BPGE_Damage.BPGE_Damage_C" 1.0 (`AbilitySystemComponent.MakeEffectContext` _returnvalue)) (struct :`TagName` "Ability.Damage") 10.0))
          (`AbilitySystemComponent.BP_ApplyGameplayEffectSpecToSelf` _returnvalue _returnvalue_2)
          (`self.K2_DestroyActor`)
          (else
            (`self.K2_DestroyActor`)))))))

(fn `UserConstructionScript`)