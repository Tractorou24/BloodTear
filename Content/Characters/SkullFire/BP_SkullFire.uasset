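; Skull Fire enemy character that shoots at its target and can strafe in a circle around it.
; BeginPlay copies tuning values into the AI blackboard, grants and configures the fire-shot ability, and plays a spawn sound.
; Tick moves it along the circle to valid AI locations, adding a gameplay tag to signal stop after the strafe duration.
; Dynamic materials provide a timeline-driven hit flash and a mouse-hover outline overlay.
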(event `self.ReceiveBeginPlay`
  (bind _mesh (`self.Mesh`))
  (bind _abilitysystemcomponent (`self.AbilitySystemComponent`))
  (`|ExecutionSequence`
    (:`then_0`
      (`BlackboardComponent.SetValueAsFloat` (`AIBlueprintHelperLibrary.GetBlackboard` null) "DetectionRange" (`self.DetectionRange`))
      (`BlackboardComponent.SetValueAsFloat` (`AIBlueprintHelperLibrary.GetBlackboard` null) "AttackRange" (`self.AttackRange`))
      (`BlackboardComponent.SetValueAsFloat` (`AIBlueprintHelperLibrary.GetBlackboard` null) "WaitAfterMoveTime" (`self.WaitAfterMoveTime`))
      (`BlackboardComponent.SetValueAsInt` (`AIBlueprintHelperLibrary.GetBlackboard` null) "MaxAttackBeforeMove" (`self.MaxAttackBeforeMove`))
      (`BlackboardComponent.SetValueAsFloat` (`AIBlueprintHelperLibrary.GetBlackboard` null) "StrafeDuration" (`self.StrafeDuration`))
      (bind _returnvalue (`AbilitySystemComponent.K2_GiveAbility` _abilitysystemcomponent "/Game/Characters/SkullFire/BPGA_SkullFireShot.BPGA_SkullFireShot_C" 0 -1))
      (bind _asbpga_skull_fire_shot (cast `/Game/Characters/SkullFire/BPGA_SkullFireShot` (`.ReturnValue` (`AbilitySystemBlueprintLibrary.GetGameplayAbilityFromSpecHandle` _abilitysystemcomponent _returnvalue))))
      (set `/Game/Characters/SkullFire/BPGA_SkullFireShot.Speed` (`self.Fire Shot Speed`) _asbpga_skull_fire_shot)
      (set `/Game/Characters/SkullFire/BPGA_SkullFireShot.Damage` (`self.ShotDamages`) _asbpga_skull_fire_shot)
      (set `/Game/Characters/SkullFire/BPGA_SkullFireShot.CastingTime` (`self.CastingTime`) _asbpga_skull_fire_shot)
      (set `EnsGameplayAbilityBase.CooldownDuration` (`self.AttackCooldown`) _asbpga_skull_fire_shot))
    (:`then_1`
      ;[0 0 0] Setup Materials Feedback
      (bind _returnvalue_2 (`KismetMaterialLibrary.CreateDynamicMaterialInstance` "/Game/Art/Materials/MasterMaterials/Outline/MM_Outline.MM_Outline"))
      (set `self.DynamicOverlayMaterial` _returnvalue_2)
      (for (_array_element _array_index) (`MeshComponent.GetMaterials` _mesh)
        (bind _returnvalue_3 (`KismetMaterialLibrary.CreateDynamicMaterialInstance` _array_element))
        (`KismetArrayLibrary.Array_Add` (`self.DynamicMaterial`) _returnvalue_3)
        (`PrimitiveComponent.SetMaterial` _mesh _array_index _returnvalue_3)))
    (:`then_2`
      ;[0 0 0] Feedback Hit
      (add `self.OnHitDelegate` (delegate `TakingDamage`)))
    (:`then_3`
      ;[0.3633 0 0.5104] FMOD - Play SkullFire Spawn
      (`FMODBlueprintStatics.PlayEventAtLocation` "/Game/FMOD/Events/SFX/Characters/FireSkulls/FS_Spawn.FS_Spawn"))))

(event `TakingDamage` :!signature `self.OnHitDelegate`
  (params (DamageAmount :type "Float (single-precision)"))
  ;[0 0 0] Feedback Hit
  (bind (_direction _newtrack_0) (`Timeline|Timeline` :!via `PlayFromStart`)
    (:`Update`
      (`MaterialInstanceDynamic.SetScalarParameterValue` (`self.DynamicMaterial`) "HitIntensity" _newtrack_0))))

(event `self.MouseInteractableComponent.OnMouseHoverStart`
  ;[0 0 0] Feedback Outline
  (`MeshComponent.SetOverlayMaterial` (`self.Mesh`) (`self.DynamicOverlayMaterial`)))

(event `self.MouseInteractableComponent.OnMouseHoverEnd`
  ;[0 0 0] Feedback Outline
  (`MeshComponent.SetOverlayMaterial` (`self.Mesh`) null))

(event `self.ReceiveTick`
  (params (DeltaSeconds :type "Float (single-precision)"))
  (`SceneComponent.K2_SetWorldRotation` (`self.UIEnemyInfoComponent`) (struct :`Pitch` 45.0 :`Yaw` 135.0) false false)
  (if (`self.IsStrafingAroundTarget`)
    (`|ExecutionSequence`
      (:`then_0`
        (`/Engine/EditorBlueprintResources/StandardMacros.DoOnce` false :!label _label
          (:`Completed`
            (`GameplayTask_WaitDelay.TaskWaitDelay` (`AIBlueprintHelperLibrary.GetAIController` self) (`self.StrafeDuration`)
              (:`OnFinish`
                (`AbilitySystemBlueprintLibrary.AddLooseGameplayTags` self (`BlueprintGameplayTagLibrary.MakeLiteralGameplayTagContainer` (struct :`GameplayTags` (struct :`(TagName` "Ability.SkullFireStrafe.Stop")))))
                (goto _label :!via `Reset`))))))
      (:`then_1`
        (bind _asactor (cast `Actor` (`BlackboardComponent.GetValueAsObject` (`AIBlueprintHelperLibrary.GetBlackboard` null) "Target")))
        (bind _result (`MathAI.GetNextPointOnCircleByAngle` (`self.K2_GetActorLocation` _asactor) (`self.K2_GetActorLocation`) (`self.StrafeSpeed`) DeltaSeconds (`self.StrafeClockWise`)))
        (if (`AIBlueprintHelperLibrary.IsValidAILocation` _result)
          (`self.K2_SetActorLocation` _result)
          (`KismetSystemLibrary.DrawDebugBox` _result (5.0 5.0 5.0) (struct) (struct) 0.01))))))

(fn `StartStrafeAroundTarget`
  (set `self.IsStrafingAroundTarget` true)
  (set `self.StrafeClockWise` (== (`KismetMathLibrary.RandomInteger` 2) 0)))

(fn `StopStrafeAroundTarget`
  (set `self.IsStrafingAroundTarget` false))

(fn `UserConstructionScript`)