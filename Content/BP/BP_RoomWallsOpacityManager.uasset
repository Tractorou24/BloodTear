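; Room manager that dissolves tagged wall meshes while the player is inside its box collision and restores them on exit.
; On BeginPlay it gathers "Disapear"-tagged meshes from actors with the room Tag and assigns shared dynamic materials to "Masked" slots, matched by name.
; Two timelines drive the Dissolve parameter, handing over mid-fade when the player turns back.
; Fully dissolved meshes are hidden until reappearing.
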(event `self.ReceiveBeginPlay`
  (bind _boxcollision (`self.BoxCollision`))
  (add `PrimitiveComponent.OnComponentBeginOverlap` _boxcollision (delegate `OnComponentBeginOverlap_Event`))
  (add `PrimitiveComponent.OnComponentEndOverlap` _boxcollision (delegate `OnComponentEndOverlap_Event`))
  (bind _outactors (`GameplayStatics.GetAllActorsWithTag` (`KismetStringLibrary.Conv_StringToName` (`self.Tag`))))
  (for _array_element _outactors
    (`KismetArrayLibrary.Array_Append` (`self.SMC`) (`self.GetComponentsByTag` _array_element "/Script/Engine.StaticMeshComponent" "Disapear")))
  (for _array_element_2 (`self.Materials_Data`)
    (bind _returnvalue (`KismetMaterialLibrary.CreateDynamicMaterialInstance` _array_element_2 (`KismetStringLibrary.Conv_StringToName` (`KismetStringLibrary.Concat_StrStr` (`KismetSystemLibrary.GetObjectName` _array_element_2) (`self.Tag`)))))
    (`KismetArrayLibrary.Array_Add` (`self.DynamicsMaterialsInstances`) _returnvalue))
  (for _array_element_3 (`self.SMC`)
    (for _index (range (`PrimitiveComponent.GetNumMaterials` _array_element_3))
      (if (== (`|GetArrayItem` (`PrimitiveComponent.GetMaterialSlotNames` _array_element_3) _index) "Masked")
        (for _array_element_4 (`self.DynamicsMaterialsInstances`)
          (if (== (`KismetSystemLibrary.GetObjectName` _array_element_4) (`KismetStringLibrary.Concat_StrStr` (`KismetSystemLibrary.GetObjectName` (`PrimitiveComponent.GetMaterial` _array_element_3 _index)) (`self.Tag`)))
            (`PrimitiveComponent.SetMaterial` _array_element_3 _index _array_element_4)
            (break)))))))

(event `OnComponentBeginOverlap_Event`
  (params (OverlappedComponent :type "PrimitiveComponent Object Reference") (OtherActor :type "Actor Object Reference") (OtherComp :type "PrimitiveComponent Object Reference") (OtherBodyIndex :type Integer) (bFromSweep :type Boolean) (SweepResult :type "HitResult Structure (by ref)"))
  (if (== OtherActor (`GameplayStatics.GetPlayerCharacter` 0))
    (set `self.HasDisapeared` true)
    (set `self.IsDisapearing` true)
    (if (`self.IsAppearing`)
      (`|ExecutionSequence`
        (:`then_0`
          (bind (_direction _dissolve) (`Timeline|Timeline_0` :`NewTime` (* (- (stale `OnComponentEndOverlap_Event` _returnvalue) 1.0) -1.0) :!via `Stop` :!label _label)
            (:`Update`
              (for _array_element (`self.DynamicsMaterialsInstances`)
                (`MaterialInstanceDynamic.SetScalarParameterValue` _array_element "Dissolve" _dissolve)))
            (:`Finished`
              (if (`self.IsDisapearing`)
                (set `self.IsAppearing` false)
                (else
                  (set `self.HasDisapeared` false)
                  (set `self.IsAppearing` false))))))
        (:`then_1`
          (bind _returnvalue (`MaterialInstanceDynamic.K2_GetScalarParameterValue` (`|GetArrayItem` (`self.DynamicsMaterialsInstances`)) "Dissolve"))
          (bind (_direction_2 _dissolve_2) (`Timeline|Timeline` :`NewTime` (* (- _returnvalue 1.0) -1.0) :!via `SetNewTime` :!label _label_2)
            (:`Update`
              (for _array_element_2 (`self.DynamicsMaterialsInstances`)
                (`MaterialInstanceDynamic.SetScalarParameterValue` _array_element_2 "Dissolve" _dissolve_2)))
            (:`Finished`
              (if (not (`self.IsAppearing`))
                (`SceneComponent.SetVisibility` (`self.SMC`) false false))
              (set `self.IsDisapearing` false))))
        (:`then_2`
          (goto _label_2)))
      (else
        (goto _label_2 :!via `PlayFromStart`)))))

(event `OnComponentEndOverlap_Event`
  (params (OverlappedComponent :type "PrimitiveComponent Object Reference") (OtherActor :type "Actor Object Reference") (OtherComp :type "PrimitiveComponent Object Reference") (OtherBodyIndex :type Integer))
  (bind _smc (`self.SMC`))
  (if (== OtherActor (`GameplayStatics.GetPlayerCharacter` 0))
    (if (`self.HasDisapeared`)
      (set `self.IsAppearing` true)
      (if (`self.IsDisapearing`)
        (`SceneComponent.SetVisibility` _smc true false)
        (`|ExecutionSequence`
          (:`then_0`
            (goto _label_2 :!via `Stop`))
          (:`then_1`
            (bind _returnvalue (`MaterialInstanceDynamic.K2_GetScalarParameterValue` (`|GetArrayItem` (`self.DynamicsMaterialsInstances`)) "Dissolve"))
            (goto _label :!via `SetNewTime`))
          (:`then_2`
            (goto _label :!via `Reverse`)))
        (else
          (`SceneComponent.SetVisibility` _smc true false)
          (goto _label :!via `ReverseFromEnd`))))))

(fn `CheckMaterialSlot`
  (params (MaterialSlotName :type Name) (StaticMeshComponent :type "StaticMeshComponent Object Reference") (MaterialToSet :type "MaterialInstanceDynamic Object Reference"))
  (if (`PrimitiveComponent.IsMaterialSlotNameValid` StaticMeshComponent MaterialSlotName)
    (`PrimitiveComponent.SetMaterialByName` StaticMeshComponent MaterialSlotName MaterialToSet)
    (return)))

(fn `UserConstructionScript`)