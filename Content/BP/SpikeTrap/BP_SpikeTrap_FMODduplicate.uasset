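; Spike trap that rises in two timeline-driven phases, preparation and hit, when a character enters its trigger, with an FMOD sound for each phase.
; Timelines offset the spikes' height from their start position, separated by a configurable delay.
; After a cooldown it fires again if characters still overlap the actor, otherwise it re-arms.
; A separate box damages characters on overlap through a set-by-caller GAS effect applied via the target's ability system.
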(event `self.ReceiveBeginPlay`
  (bind (_relativelocation_x _relativelocation_y _relativelocation_z) (`KismetMathLibrary.BreakVector` (`SceneComponent.RelativeLocation` (`self.Spikes`))))
  (add `PrimitiveComponent.OnComponentBeginOverlap` (`self.OverlapTrap`) (delegate `TrapShouldActivate`))
  (add `PrimitiveComponent.OnComponentBeginOverlap` (`self.Box`) (delegate `OnBoxShouldDamage`))
  (set `self.StartPosition` (`KismetMathLibrary.MakeVector` _relativelocation_x _relativelocation_y _relativelocation_z)))

(event `OnBoxShouldDamage`
  (params (OverlappedComponent :type "PrimitiveComponent Object Reference") (OtherActor :type "Actor Object Reference") (OtherComp :type "PrimitiveComponent Object Reference") (OtherBodyIndex :type Integer) (bFromSweep :type Boolean) (SweepResult :type "HitResult Structure (by ref)"))
  (bind _asens_character_base (cast `EnsCharacterBase` OtherActor))
  (`self.GiveDamage` _asens_character_base 10.0))

(event `TrapShouldActivate`
  (params (OverlappedComponent :type "PrimitiveComponent Object Reference") (OtherActor :type "Actor Object Reference") (OtherComp :type "PrimitiveComponent Object Reference") (OtherBodyIndex :type Integer) (bFromSweep :type Boolean) (SweepResult :type "HitResult Structure (by ref)"))
  (if (`GameplayStatics.ObjectIsA` OtherActor "/Script/ENS.EnsCharacterBase")
    (if (not (`self.IsActivating?`))
      (set `self.IsActivating?` true)
      (`|ExecutionSequence` :!label _label
        (:`then_0`
          (bind (_direction _elevation) (`Timeline|Preparation` :!via `PlayFromStart`)
            (:`Update`
              (`SceneComponent.K2_SetRelativeLocation` (`self.Spikes`) (`KismetMathLibrary.MakeVector` (.x (`self.StartPosition`)) (.y (`self.StartPosition`)) (+ (.z (`self.StartPosition`)) _elevation)) false false))
            (:`Finished`
              (`KismetSystemLibrary.Delay` (`self.DelayAttack`))
              (`|ExecutionSequence`
                (:`then_0`
                  (bind (_direction_2 _elevation_2) (`Timeline|Hit` :!via `PlayFromStart`)
                    (:`Update`
                      (`SceneComponent.K2_SetRelativeLocation` (`self.Spikes`) (`KismetMathLibrary.MakeVector` (.x (`self.StartPosition`)) (.y (`self.StartPosition`)) (+ (.z (`self.StartPosition`)) _elevation_2)) false false))
                    (:`Finished`
                      (`KismetSystemLibrary.Delay` (`self.DelayCanBeReactivated`))
                      (if (!= (`KismetArrayLibrary.Array_Length` (`self.GetOverlappingActors` "/Script/ENS.EnsCharacterBase")) 0)
                        (`self.TrapReactivation`)
                        (else
                          (set `self.IsActivating?` false))))))
                (:`then_1`
                  ;[0.3633 0 0.5104] FMOD - Play Trap Activating
                  (`FMODBlueprintStatics.PlayEventAtLocation` "/Game/FMOD/Events/SFX/Enviro/Enviro_SpikeTrapsActivating.Enviro_SpikeTrapsActivating" (`KismetMathLibrary.MakeTransform` (`self.K2_GetActorLocation` self))))))))
        (:`then_1`
          ;[0.3633 0 0.5104] FMOD - Play Trap Preparing
          (`FMODBlueprintStatics.PlayEventAtLocation` "/Game/FMOD/Events/SFX/Enviro/Enviro_SpikeTrapsPreparing.Enviro_SpikeTrapsPreparing" (`KismetMathLibrary.MakeTransform` (`self.K2_GetActorLocation` self))))))))

(event `TrapReactivation`
  (goto _label))

(fn `GiveDamage`
  (params (Target :type "EnsCharacterBase Object Reference") (Damage :type "Float (double-precision)"))
  (bind _returnvalue (`AbilitySystemBlueprintLibrary.GetAbilitySystemComponent` Target))
  (bind _returnvalue_2 (`AbilitySystemBlueprintLibrary.AssignTagSetByCallerMagnitude` (`AbilitySystemComponent.MakeOutgoingSpec` _returnvalue "/Game/Characters/Player/Abilities/DevelopperTests/BPGE_Damage.BPGE_Damage_C" 0.0 (`AbilitySystemComponent.MakeEffectContext` _returnvalue)) (struct :`TagName` "Ability.Damage") Damage))
  (`AbilitySystemComponent.BP_ApplyGameplayEffectSpecToSelf` _returnvalue _returnvalue_2)
  (return))

(fn `UserConstructionScript`)