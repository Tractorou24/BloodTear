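; Crystal transition actor that changes the look of a tagged crystal room's crystals when one of its fence doors signals opening, treated as combat finished.
; On BeginPlay it binds to the tagged doors and creates shared dynamic crystal materials, assigned to tagged actors' meshes by matching first slot name to instance name.
; The door event plays a timeline on Highlight, switches Transition on, then runs a second Highlight timeline.
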(event `self.ReceiveBeginPlay`
  (bind _crystalroomtag (`self.CrystalRoomTag`))
  (bind _outactors (`GameplayStatics.GetAllActorsOfClassWithTag` "/Game/BP/Doors/FenceDoorCorridor02/BP_FenceDoor.BP_FenceDoor_C" (`KismetStringLibrary.Conv_StringToName` _crystalroomtag)))
  (for _array_element _outactors
    (add `/Game/BP/Doors/FenceDoorCorridor02/BP_FenceDoor.DoorIsOpening` _array_element (delegate `CombatFinished`)))
  (bind _returnvalue (`KismetMaterialLibrary.CreateDynamicMaterialInstance` "/Game/Art/Materials/ComplexMaterials/M_LittleCrystalAtlas01.M_LittleCrystalAtlas01" (`KismetStringLibrary.Conv_StringToName` (`KismetStringLibrary.Concat_StrStr` _crystalroomtag "LittleCrystalAtlas01"))))
  (`KismetArrayLibrary.Array_Add` (`self.DynamicMaterials`) _returnvalue)
  (bind _returnvalue_2 (`KismetMaterialLibrary.CreateDynamicMaterialInstance` "/Game/Art/Materials/ComplexMaterials/MI_LittleCrystalAtlas02.MI_LittleCrystalAtlas02" (`KismetStringLibrary.Conv_StringToName` (`KismetStringLibrary.Concat_StrStr` _crystalroomtag "LittleCrystalAtlas02"))))
  (`KismetArrayLibrary.Array_Add` (`self.DynamicMaterials`) _returnvalue_2)
  (bind _returnvalue_3 (`KismetMaterialLibrary.CreateDynamicMaterialInstance` "/Game/Art/Materials/ComplexMaterials/MI_BigCrystalB.MI_BigCrystalB" (`KismetStringLibrary.Conv_StringToName` (`KismetStringLibrary.Concat_StrStr` _crystalroomtag "BigCrystalB"))))
  (`KismetArrayLibrary.Array_Add` (`self.DynamicMaterials`) _returnvalue_3)
  (bind _returnvalue_4 (`KismetMaterialLibrary.CreateDynamicMaterialInstance` "/Game/Art/Materials/ComplexMaterials/MI_MRCrystalA.MI_MRCrystalA" (`KismetStringLibrary.Conv_StringToName` (`KismetStringLibrary.Concat_StrStr` _crystalroomtag "MRCrystalA"))))
  (`KismetArrayLibrary.Array_Add` (`self.DynamicMaterials`) _returnvalue_4)
  ;[0 0 0] MaterialSetCrystal
  (bind _outactors_2 (`GameplayStatics.GetAllActorsWithTag` (`KismetStringLibrary.Conv_StringToName` (`self.CrystalRoomTag`))))
  (for _array_element_2 _outactors_2
    (for _array_element_3 (`self.K2_GetComponentsByClass` _array_element_2 "/Script/Engine.StaticMeshComponent")
      (for _array_element_4 (`self.DynamicMaterials`)
        (if (`KismetStringLibrary.EqualEqual_StrStr` (`KismetSystemLibrary.GetObjectName` _array_element_4) (`KismetStringLibrary.Concat_StrStr` (`self.CrystalRoomTag`) (`KismetStringLibrary.Conv_NameToString` (`|GetArrayItem` (`PrimitiveComponent.GetMaterialSlotNames` _array_element_3)))))
          (`PrimitiveComponent.SetMaterial` _array_element_3 0 _array_element_4)
          (break))))))

(event `CombatFinished`
  (bind _dynamicmaterials (`self.DynamicMaterials`))
  (bind (_direction _transition) (`Timeline|Timeline` :!via `PlayFromStart`)
    (:`Update`
      (`MaterialInstanceDynamic.SetScalarParameterValue` _dynamicmaterials "Highlight" _transition))
    (:`Finished`
      (`MaterialInstanceDynamic.SetScalarParameterValue` _dynamicmaterials "Transition" 1.0)
      (bind (_direction_2 _highlightvalue) (`Timeline|Timeline_0` :!via `PlayFromStart`)
        (:`Update`
          (`MaterialInstanceDynamic.SetScalarParameterValue` _dynamicmaterials "Highlight" _highlightvalue))))))

(fn `UserConstructionScript`)