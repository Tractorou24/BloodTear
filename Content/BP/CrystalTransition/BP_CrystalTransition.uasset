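; Floating arena crystal that plays the end-of-level purification when a tagged BP_MultiAreaSpawner finishes (debug key J also triggers it).
; BeginPlay assigns shared dynamic materials to near, mid and far tagged crystals by slot name and starts looping-style timeline float and orbit motion.
; The transition staggers highlight timelines across those groups, swaps VFX, materials and lights to pure, plays the EndLevel sequence, then opens BP_HellDoor and pauses on the ending widget.
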(event Custom|FloatingStart
  (bind _pivot_crystal (Variables|Default|GetPivot_Crystal))
  (bind _startinglocation_orbitingcrystal01 (Variables|Default|GetStartingLocation_OrbitingCrystal01))
  (bind _startingrotation_orbitingcrystal01 (Variables|Default|GetStartingRotation_OrbitingCrystal01))
  (bind _startinglocation_orbitingcrystal02 (Variables|Default|GetStartingLocation_OrbitingCrystal02))
  (bind _startingrotation_orbitingcrystal02 (Variables|Default|GetStartingRotation_OrbitingCrystal02))
  (bind _startinglocation_orbitingcrystal03 (Variables|Default|GetStartingLocation_OrbitingCrystal03))
  (bind _pivot_orbitingcrystal01 (Variables|Default|GetPivot_OrbitingCrystal01))
  (bind _pivot_orbitingcrystal03 (Variables|Default|GetPivot_OrbitingCrystal03))
  (bind _startinglocation_crystal (Variables|Default|GetStartingLocation_Crystal))
  (bind _startingrotation_orbitingcrystal03 (Variables|Default|GetStartingRotation_OrbitingCrystal03))
  (bind _pivot_orbitingcrystal02 (Variables|Default|GetPivot_OrbitingCrystal02))
  ;[0 0 0] FloatingAnimation
  (Utilities|FlowControl|Sequence
    (:then_0
      (bind _translation (Timeline|CurveTranslation PlayFromStart)
        (:Update
          (Transformation|SetRelativeLocation _pivot_crystal (Math|Vector|MakeVector (+ (.x _startinglocation_crystal) (.x _translation)) (+ (.y _startinglocation_crystal) (.y _translation)) (+ (.z _startinglocation_crystal) (.z _translation))) false false))))
    (:then_1
      (bind _rotation (Timeline|CrystalRotation PlayFromStart)
        (:Update
          (Transformation|SetRelativeRotation _pivot_crystal (Math|Rotator|MakeRotator (.x _rotation) (.y _rotation) (.z _rotation)) false false))))
    (:then_2
      (bind _translation_2 (Timeline|OrbitingCrystal01_Translation PlayFromStart)
        (:Update
          (Transformation|SetRelativeLocation _pivot_orbitingcrystal01 (Math|Vector|MakeVector (+ (.x _startinglocation_orbitingcrystal01) (.x _translation_2)) (+ (.y _startinglocation_orbitingcrystal01) (.y _translation_2)) (+ (.z _startinglocation_orbitingcrystal01) (.z _translation_2))) false false))))
    (:then_3
      (bind _rotation_2 (Timeline|OrbitingCrystals PlayFromStart)
        (:Update
          (Transformation|SetRelativeRotation (Variables|Default|GetPivot_OrbitingCrystals) (Math|Rotator|MakeRotator 0.0 0.0 _rotation_2) false false))))
    (:then_4
      (bind _rotation_3 (Timeline|OrbitingCrystal01_Rotation PlayFromStart)
        (:Update
          (Transformation|SetRelativeRotation _pivot_orbitingcrystal01 (Math|Rotator|MakeRotator (+ (.x _startingrotation_orbitingcrystal01) (.x _rotation_3)) (+ (.y _startingrotation_orbitingcrystal01) (.y _rotation_3)) (+ (.z _startingrotation_orbitingcrystal01) (.z _rotation_3))) false false))))
    (:then_5
      (Utilities|FlowControl|Delay 1.0)
      (bind _translation_3 (Timeline|OrbitingCrystal02_Translation PlayFromStart)
        (:Update
          (Transformation|SetRelativeLocation _pivot_orbitingcrystal02 (Math|Vector|MakeVector (+ (.x _startinglocation_orbitingcrystal02) (.x _translation_3)) (+ (.y _startinglocation_orbitingcrystal02) (.y _translation_3)) (+ (.z _startinglocation_orbitingcrystal02) (.z _translation_3))) false false))))
    (:then_6
      (Utilities|FlowControl|Delay 1.0)
      (bind _rotation_4 (Timeline|OrbitingCrystal02_Rotation PlayFromStart)
        (:Update
          (Transformation|SetRelativeRotation _pivot_orbitingcrystal02 (Math|Rotator|MakeRotator (+ (.x _startingrotation_orbitingcrystal02) (.x _rotation_4)) (+ (.y _startingrotation_orbitingcrystal02) (.y _rotation_4)) (+ (.z _startingrotation_orbitingcrystal02) (.z _rotation_4))) false false))))
    (:then_7
      (Utilities|FlowControl|Delay 2.0)
      (bind _translation_4 (Timeline|OrbitingCrystal03_Translation PlayFromStart)
        (:Update
          (Transformation|SetRelativeLocation _pivot_orbitingcrystal03 (Math|Vector|MakeVector (+ (.x _startinglocation_orbitingcrystal03) (.x _translation_4)) (+ (.y _startinglocation_orbitingcrystal03) (.y _translation_4)) (+ (.z _startinglocation_orbitingcrystal03) (.z _translation_4))) false false))))
    (:then_8
      (Utilities|FlowControl|Delay 2.0)
      (bind _rotation_5 (Timeline|OrbitingCrystal03_Rotation PlayFromStart)
        (:Update
          (Transformation|SetRelativeRotation _pivot_orbitingcrystal03 (Math|Rotator|MakeRotator (+ (.x _startingrotation_orbitingcrystal03) (.x _rotation_5)) (+ (.y _startingrotation_orbitingcrystal03) (.y _rotation_5)) (+ (.z _startingrotation_orbitingcrystal03) (.z _rotation_5))) false false))))))

(event Custom|StartTransition
  (bind _arenapointlights01 (Variables|Default|GetArenaPointLights01))
  (bind _output (Utilities|Array|Get(acopy) _arenapointlights01))
  (bind _pointlightcomponent (Variables|/Script/Engine.PointLight|GetPointLightComponent _output))
  ;[0 0 0] TransitionAnimation
  (Utilities|FlowControl|Sequence
    (:then_0
      (Default|CallArenaFinished)
      (bind _foundwidgets (Widget|GetAllWidgetsOfClass "/Game/Widget/WB_PlayerInfo.WB_PlayerInfo_C" true))
      (for _array_element _foundwidgets
        (Widget|RemovefromParent _array_element)))
    (:then_1
      (bind _outactors (Actor|GetAllActorsOfClasswithTag "/Script/CinematicCamera.CineCameraActor" "EndLevel"))
      (for _array_element_2 _outactors
        (Components|Activation|SetActive (Variables|/Script/Engine.CameraActor|GetCameraComponent _array_element_2) false false))
      (bind _outactors_2 (Actor|GetAllActorsOfClasswithTag "/Script/LevelSequence.LevelSequenceActor" "EndLevel"))
      (for _array_element_3 _outactors_2
        (Sequencer|Player|Play (Variables|/Script/LevelSequence.LevelSequenceActor|GetSequencePlayer _array_element_3) :!class /Script/MovieScene.MovieSceneSequencePlayer))
      (Components|Activation|Activate (Variables|Default|GetVFX_Transition) false)
      (Utilities|FlowControl|Delay 0.2)
      (Utilities|FlowControl|Sequence
        (:then_0
          (bind _transition (Timeline|StartHighlight PlayFromStart)
            (:Update
              (Rendering|Material|SetScalarParameterValue (Variables|Default|GetCrystalDynamicMaterial_01) "Highlight" _transition :!class /Script/Engine.MaterialInstanceDynamic))
            (:Finished
              (Rendering|Material|SetScalarParameterValue (Variables|Default|GetCrystalDynamicMaterial_01) "Transition" 1.0 :!class /Script/Engine.MaterialInstanceDynamic)
              (bind _highlightvalue (Timeline|EndHighlight PlayFromStart)
                (:Update
                  (Rendering|Material|SetScalarParameterValue (Variables|Default|GetCrystalDynamicMaterial_01) "Highlight" _highlightvalue :!class /Script/Engine.MaterialInstanceDynamic))
                (:Finished
                  ;[0 0 0] TransitionCrystalVFX
                  (Class|NiagaraComponent|SetAsset (Variables|Default|GetVFX) "/Game/Art/FX/Environmentals/ArenaCrystal/NS_AuraCrystalArenaPure.NS_AuraCrystalArenaPure" true)
                  (Class|NiagaraComponent|SetAsset (Variables|Default|GetVFX_OrbitingCrystal03) "/Game/Art/FX/Environmentals/ArenaCrystal/NS_OrbitingCrystalsPure.NS_OrbitingCrystalsPure" true)
                  (Rendering|Material|SetMaterial (Variables|Default|GetSM_GroundPattern) 0 "/Game/Art/FX/Environmentals/ArenaCrystal/M_GroundPattern_Pure.M_GroundPattern_Pure")
                  ;[0 0 0] TransitionElevatingAura
                  (Rendering|Material|SetMaterial (Variables|Default|GetSM_ElevatingAura) 0 "/Game/Art/FX/Environmentals/ArenaCrystal/M_ElevatingCrystalAura_Pure.M_ElevatingCrystalAura_Pure")
                  ;[0 0 0] ActivationVFXPurified
                  (Components|Activation|Activate (Variables|Default|GetVFX_ArenaPurified) true)
                  ;[0 0 0] SetValueLights
                  (Rendering|Components|Light|SetLightColor _pointlightcomponent "(R=0.137255,G=0.666667,B=1.000000,A=1.000000)" true)
                  (Rendering|Components|Light|SetLightColor (Variables|/Script/Engine.PointLight|GetPointLightComponent (Utilities|Array|Get(acopy) (Variables|Default|GetArenaPointLights02))) "(R=0.650980,G=0.729412,B=1.000000,A=1.000000)" true)
                  (Class|LightComponent|SetTemperature _pointlightcomponent 1.2e+04))))))
        (:then_1
          (Utilities|FlowControl|Delay 0.3)
          (bind _transition_2 (Timeline|Timeline PlayFromStart)
            (:Update
              (Rendering|Material|SetScalarParameterValue (Variables|Default|GetCrystalDynamicMaterial_02) "Highlight" _transition_2 :!class /Script/Engine.MaterialInstanceDynamic))
            (:Finished
              (Rendering|Material|SetScalarParameterValue (Variables|Default|GetCrystalDynamicMaterial_02) "Transition" 1.0 :!class /Script/Engine.MaterialInstanceDynamic)
              (bind _highlightvalue_2 (Timeline|Timeline_0 PlayFromStart)
                (:Update
                  (Rendering|Material|SetScalarParameterValue (Variables|Default|GetCrystalDynamicMaterial_02) "Highlight" _highlightvalue_2 :!class /Script/Engine.MaterialInstanceDynamic))))))
        (:then_2
          (Utilities|FlowControl|Delay 0.5)
          (bind _transition_3 (Timeline|Timeline_1 PlayFromStart)
            (:Update
              (Rendering|Material|SetScalarParameterValue (Variables|Default|GetCrystalDynamicMaterial_03) "Highlight" _transition_3 :!class /Script/Engine.MaterialInstanceDynamic))
            (:Finished
              (Rendering|Material|SetScalarParameterValue (Variables|Default|GetCrystalDynamicMaterial_03) "Transition" 1.0 :!class /Script/Engine.MaterialInstanceDynamic)
              (bind _highlightvalue_3 (Timeline|Timeline_2 PlayFromStart)
                (:Update
                  (Rendering|Material|SetScalarParameterValue (Variables|Default|GetCrystalDynamicMaterial_03) "Highlight" _highlightvalue_3 :!class /Script/Engine.MaterialInstanceDynamic))))))))
    (:then_2
      (bind _returnvalue (Actor|GetActorOfClass "/Game/Art/Tools/HellDoor/BP_HellDoor.BP_HellDoor_C"))
      (Utilities|FlowControl|Delay 9.0)
      (Default|EndGameDoorAnimation _returnvalue))
    (:then_3
      ;;[0 0 0] WidgetEndGame
      (Utilities|FlowControl|Delay 11.5)
      (Game|SetGamePaused true)
      (bind _returnvalue_2 (UserInterface|CreateWidget "/Game/Widget/WB_Ending.WB_Ending_C"))
      (UserInterface|Viewport|AddtoViewport _returnvalue_2 0))))

(event Custom|SpawnerFInished
  ;[0 0 0] UpdateDataSpawner
  (CallFunction|StartTransition))

(event EventBeginPlay
  (bind _crystaldynamicmaterial_01 (Variables|Default|GetCrystalDynamicMaterial_01))
  (bind _crystaldynamicmaterial_02 (Variables|Default|GetCrystalDynamicMaterial_02))
  (bind _crystaldynamicmaterial_01_2 (Variables|Default|GetCrystalDynamicMaterial_01))
  (bind _crystaldynamicmaterial_03 (Variables|Default|GetCrystalDynamicMaterial_03))
  ;[0 0 0] GetSpawnerData
  (bind _outactors (Actor|GetAllActorsOfClasswithTag "/Game/BP/Spawner/BP_MultiAreaSpawner.BP_MultiAreaSpawner_C" (Variables|Default|GetSpawnerTag)))
  (for _array_element _outactors
    (EventDispatchers|BindEventtoOnSpawnerFinished _array_element (delegate Custom|SpawnerFInished)))
  ;[0 0 0] GetArenaLights
  (bind _outactors_2 (Actor|GetAllActorsOfClasswithTag "/Script/Engine.PointLight" "ArenaLights01"))
  (Variables|Default|SetArenaPointLights01 _outactors_2)
  (bind _outactors_3 (Actor|GetAllActorsOfClasswithTag "/Script/Engine.PointLight" "ArenaLights02"))
  (Variables|Default|SetArenaPointLights02 _outactors_3)
  (bind _outactors_4 (Actor|GetAllActorsOfClasswithTag "/Script/Engine.PostProcessVolume" "Arene"))
  (Variables|Default|SetArenaPostProcess _outactors_4)
  ;[0 0 0] NearLittleCrystalsMaterialSet
  (bind _returnvalue (Rendering|Material|CreateDynamicMaterialInstance "/Game/Art/Materials/ComplexMaterials/M_LittleCrystalAtlas01.M_LittleCrystalAtlas01" "LittleCrystalAtlas01_NearTransition" "None" :!class /Script/Engine.KismetMaterialLibrary))
  (Utilities|Array|Add _crystaldynamicmaterial_01_2 _returnvalue)
  (bind _returnvalue_2 (Rendering|Material|CreateDynamicMaterialInstance "/Game/Art/Materials/ComplexMaterials/MI_LittleCrystalAtlas02.MI_LittleCrystalAtlas02" "LittleCrystalAtlas02_NearTransition" "None" :!class /Script/Engine.KismetMaterialLibrary))
  (Utilities|Array|Add _crystaldynamicmaterial_01_2 _returnvalue_2)
  (bind _returnvalue_3 (Rendering|Material|CreateDynamicMaterialInstance "/Game/Art/Materials/ComplexMaterials/MI_BigCrystalB_Arena.MI_BigCrystalB_Arena" "BigCrystalB_NearTransition" "None" :!class /Script/Engine.KismetMaterialLibrary))
  (Utilities|Array|Add _crystaldynamicmaterial_01_2 _returnvalue_3)
  (bind _outactors_5 (Actor|GetAllActorswithTag (Utilities|String|StringToName "NearArenaCrystals")))
  (for _array_element_2 _outactors_5
    (for _array_element_3 (Actor|GetComponentsByClass _array_element_2 "/Script/Engine.StaticMeshComponent")
      (bind _array_element_4 (Utilities|Array|ForEachLoopwithBreak (Variables|Default|GetCrystalDynamicMaterial_01) :!label _label)
        (:LoopBody
          (if (Utilities|Enum|Equal(Enum) (Utilities|GetObjectName _array_element_4) (Utilities|String|Append (Utilities|String|ToString(Name) (Utilities|Array|Get(acopy) (Class|PrimitiveComponent|GetMaterialSlotNames _array_element_3))) "_NearTransition"))
            (Rendering|Material|SetMaterial _array_element_3 0 _array_element_4)
            (goto _label Break))))))
  ;[0 0 0] LittleCrystalsMaterialSet
  (bind _returnvalue_4 (Rendering|Material|CreateDynamicMaterialInstance "/Game/Art/Materials/ComplexMaterials/M_LittleCrystalAtlas01.M_LittleCrystalAtlas01" "LittleCrystalAtlas01_Transition" "None" :!class /Script/Engine.KismetMaterialLibrary))
  (Utilities|Array|Add _crystaldynamicmaterial_02 _returnvalue_4)
  (bind _returnvalue_5 (Rendering|Material|CreateDynamicMaterialInstance "/Game/Art/Materials/ComplexMaterials/MI_LittleCrystalAtlas02.MI_LittleCrystalAtlas02" "LittleCrystalAtlas02_Transition" "None" :!class /Script/Engine.KismetMaterialLibrary))
  (Utilities|Array|Add _crystaldynamicmaterial_02 _returnvalue_5)
  (bind _returnvalue_6 (Rendering|Material|CreateDynamicMaterialInstance "/Game/Art/Materials/ComplexMaterials/MI_BigCrystalB_Arena.MI_BigCrystalB_Arena" "BigCrystalB_Transition" "None" :!class /Script/Engine.KismetMaterialLibrary))
  (Utilities|Array|Add _crystaldynamicmaterial_02 _returnvalue_6)
  (bind _outactors_6 (Actor|GetAllActorswithTag (Utilities|String|StringToName "ArenaCrystals")))
  (for _array_element_5 _outactors_6
    (for _array_element_6 (Actor|GetComponentsByClass _array_element_5 "/Script/Engine.StaticMeshComponent")
      (bind _array_element_7 (Utilities|Array|ForEachLoopwithBreak (Variables|Default|GetCrystalDynamicMaterial_02) :!label _label_2)
        (:LoopBody
          (if (Utilities|Enum|Equal(Enum) (Utilities|GetObjectName _array_element_7) (Utilities|String|Append (Utilities|String|ToString(Name) (Utilities|Array|Get(acopy) (Class|PrimitiveComponent|GetMaterialSlotNames _array_element_6))) "_Transition"))
            (Rendering|Material|SetMaterial _array_element_6 0 _array_element_7)
            (goto _label_2 Break))))))
  ;[0 0 0] NearLittleCrystalsMaterialSet
  (bind _returnvalue_7 (Rendering|Material|CreateDynamicMaterialInstance "/Game/Art/Materials/ComplexMaterials/M_LittleCrystalAtlas01.M_LittleCrystalAtlas01" "LittleCrystalAtlas01_FarTransition" "None" :!class /Script/Engine.KismetMaterialLibrary))
  (Utilities|Array|Add _crystaldynamicmaterial_03 _returnvalue_7)
  (bind _returnvalue_8 (Rendering|Material|CreateDynamicMaterialInstance "/Game/Art/Materials/ComplexMaterials/MI_LittleCrystalAtlas02.MI_LittleCrystalAtlas02" "LittleCrystalAtlas02_FarTransition" "None" :!class /Script/Engine.KismetMaterialLibrary))
  (Utilities|Array|Add _crystaldynamicmaterial_03 _returnvalue_8)
  (bind _returnvalue_9 (Rendering|Material|CreateDynamicMaterialInstance "/Game/Art/Materials/ComplexMaterials/MI_BigCrystalB_Arena.MI_BigCrystalB_Arena" "BigCrystalB_FarTransition" "None" :!class /Script/Engine.KismetMaterialLibrary))
  (Utilities|Array|Add _crystaldynamicmaterial_03 _returnvalue_9)
  (bind _outactors_7 (Actor|GetAllActorswithTag (Utilities|String|StringToName "FarArenaCrystals")))
  (for _array_element_8 _outactors_7
    (for _array_element_9 (Actor|GetComponentsByClass _array_element_8 "/Script/Engine.StaticMeshComponent")
      (bind _array_element_10 (Utilities|Array|ForEachLoopwithBreak (Variables|Default|GetCrystalDynamicMaterial_03) :!label _label_3)
        (:LoopBody
          (if (Utilities|Enum|Equal(Enum) (Utilities|GetObjectName _array_element_10) (Utilities|String|Append (Utilities|String|ToString(Name) (Utilities|Array|Get(acopy) (Class|PrimitiveComponent|GetMaterialSlotNames _array_element_9))) "_FarTransition"))
            (Rendering|Material|SetMaterial _array_element_9 0 _array_element_10)
            (goto _label_3 Break))))))
  ;[0 0 0] Floating_CrystalMaterialSet
  (bind _returnvalue_10 (Rendering|Material|CreateDynamicMaterialInstance "/Game/Art/Materials/ComplexMaterials/M_CrystalArena.M_CrystalArena" "None" "None" :!class /Script/Engine.KismetMaterialLibrary))
  (Utilities|Array|Add (Variables|Default|GetCrystalDynamicMaterial_01) _returnvalue_10)
  (Rendering|Material|SetMaterial (Variables|Default|GetSM_Crystal) 0 _returnvalue_10)
  ;[0 0 0] Floating_LittleCrystalsMaterialSet
  (bind _returnvalue_11 (Rendering|Material|CreateDynamicMaterialInstance "/Game/Art/Materials/ComplexMaterials/M_LittleCrystalAtlas01_Arena.M_LittleCrystalAtlas01_Arena" "LittleCrystalAtlas01_Floating_Transition" "None" :!class /Script/Engine.KismetMaterialLibrary))
  (Utilities|Array|Add _crystaldynamicmaterial_01 _returnvalue_11)
  (bind _returnvalue_12 (Rendering|Material|CreateDynamicMaterialInstance "/Game/Art/Materials/ComplexMaterials/MI_LittleCrystalAtlas02_Arena.MI_LittleCrystalAtlas02_Arena" "LittleCrystalAtlas02_Floating_Transition" "None" :!class /Script/Engine.KismetMaterialLibrary))
  (Utilities|Array|Add _crystaldynamicmaterial_01 _returnvalue_12)
  (for _array_element_11 (Utilities|Array|MakeArray (Variables|Default|GetSM_OrbitingCrystal01) (Variables|Default|GetSM_OrbitingCrystal02) (Variables|Default|GetSM_OrbitingCrystal03))
    (bind _array_element_12 (Utilities|Array|ForEachLoopwithBreak (Variables|Default|GetCrystalDynamicMaterial_01) :!label _label_4)
      (:LoopBody
        (if (Utilities|Enum|Equal(Enum) (Utilities|GetObjectName _array_element_12) (Utilities|String|Append (Utilities|String|ToString(Name) (Utilities|Array|Get(acopy) (Class|PrimitiveComponent|GetMaterialSlotNames _array_element_11))) "_Floating_Transition"))
          (Rendering|Material|SetMaterial _array_element_11 0 _array_element_12)
          (goto _label_4 Break)))))
  (CallFunction|FloatingStart))

(event Input|KeyboardEvents|DebugKeyJ
  (params (Key :type Key%20Structure :default "None") (ActionValue :type Input%20Action%20Value%20Structure))
  (bind _arenapointlights01 (Variables|Default|GetArenaPointLights01))
  (bind _output (Utilities|Array|Get(acopy) _arenapointlights01))
  (bind _pointlightcomponent (Variables|/Script/Engine.PointLight|GetPointLightComponent _output))
  ;[0 0 0] TransitionAnimation
  (:Pressed
    (Utilities|FlowControl|Sequence
      (:then_0
        (Default|CallArenaFinished)
        (bind _foundwidgets (Widget|GetAllWidgetsOfClass "/Game/Widget/WB_PlayerInfo.WB_PlayerInfo_C" true))
        (for _array_element _foundwidgets
          (Widget|RemovefromParent _array_element)))
      (:then_1
        (bind _outactors (Actor|GetAllActorsOfClasswithTag "/Script/CinematicCamera.CineCameraActor" "EndLevel"))
        (for _array_element_2 _outactors
          (Components|Activation|SetActive (Variables|/Script/Engine.CameraActor|GetCameraComponent _array_element_2) false false))
        (bind _outactors_2 (Actor|GetAllActorsOfClasswithTag "/Script/LevelSequence.LevelSequenceActor" "EndLevel"))
        (for _array_element_3 _outactors_2
          (Sequencer|Player|Play (Variables|/Script/LevelSequence.LevelSequenceActor|GetSequencePlayer _array_element_3) :!class /Script/MovieScene.MovieSceneSequencePlayer))
        (Components|Activation|Activate (Variables|Default|GetVFX_Transition) false)
        (Utilities|FlowControl|Delay 0.2)
        (Utilities|FlowControl|Sequence
          (:then_0
            (bind _transition (Timeline|StartHighlight PlayFromStart)
              (:Update
                (Rendering|Material|SetScalarParameterValue (Variables|Default|GetCrystalDynamicMaterial_01) "Highlight" _transition :!class /Script/Engine.MaterialInstanceDynamic))
              (:Finished
                (Rendering|Material|SetScalarParameterValue (Variables|Default|GetCrystalDynamicMaterial_01) "Transition" 1.0 :!class /Script/Engine.MaterialInstanceDynamic)
                (bind _highlightvalue (Timeline|EndHighlight PlayFromStart)
                  (:Update
                    (Rendering|Material|SetScalarParameterValue (Variables|Default|GetCrystalDynamicMaterial_01) "Highlight" _highlightvalue :!class /Script/Engine.MaterialInstanceDynamic))
                  (:Finished
                    ;[0 0 0] TransitionCrystalVFX
                    (Class|NiagaraComponent|SetAsset (Variables|Default|GetVFX) "/Game/Art/FX/Environmentals/ArenaCrystal/NS_AuraCrystalArenaPure.NS_AuraCrystalArenaPure" true)
                    (Class|NiagaraComponent|SetAsset (Variables|Default|GetVFX_OrbitingCrystal03) "/Game/Art/FX/Environmentals/ArenaCrystal/NS_OrbitingCrystalsPure.NS_OrbitingCrystalsPure" true)
                    (Rendering|Material|SetMaterial (Variables|Default|GetSM_GroundPattern) 0 "/Game/Art/FX/Environmentals/ArenaCrystal/M_GroundPattern_Pure.M_GroundPattern_Pure")
                    ;[0 0 0] TransitionElevatingAura
                    (Rendering|Material|SetMaterial (Variables|Default|GetSM_ElevatingAura) 0 "/Game/Art/FX/Environmentals/ArenaCrystal/M_ElevatingCrystalAura_Pure.M_ElevatingCrystalAura_Pure")
                    ;[0 0 0] ActivationVFXPurified
                    (Components|Activation|Activate (Variables|Default|GetVFX_ArenaPurified) true)
                    ;[0 0 0] SetValueLights
                    (Rendering|Components|Light|SetLightColor _pointlightcomponent "(R=0.137255,G=0.666667,B=1.000000,A=1.000000)" true)
                    (Rendering|Components|Light|SetLightColor (Variables|/Script/Engine.PointLight|GetPointLightComponent (Utilities|Array|Get(acopy) (Variables|Default|GetArenaPointLights02))) "(R=0.650980,G=0.729412,B=1.000000,A=1.000000)" true)
                    (Class|LightComponent|SetTemperature _pointlightcomponent 1.2e+04))))))
          (:then_1
            (Utilities|FlowControl|Delay 0.3)
            (bind _transition_2 (Timeline|Timeline PlayFromStart)
              (:Update
                (Rendering|Material|SetScalarParameterValue (Variables|Default|GetCrystalDynamicMaterial_02) "Highlight" _transition_2 :!class /Script/Engine.MaterialInstanceDynamic))
              (:Finished
                (Rendering|Material|SetScalarParameterValue (Variables|Default|GetCrystalDynamicMaterial_02) "Transition" 1.0 :!class /Script/Engine.MaterialInstanceDynamic)
                (bind _highlightvalue_2 (Timeline|Timeline_0 PlayFromStart)
                  (:Update
                    (Rendering|Material|SetScalarParameterValue (Variables|Default|GetCrystalDynamicMaterial_02) "Highlight" _highlightvalue_2 :!class /Script/Engine.MaterialInstanceDynamic))))))
          (:then_2
            (Utilities|FlowControl|Delay 0.5)
            (bind _transition_3 (Timeline|Timeline_1 PlayFromStart)
              (:Update
                (Rendering|Material|SetScalarParameterValue (Variables|Default|GetCrystalDynamicMaterial_03) "Highlight" _transition_3 :!class /Script/Engine.MaterialInstanceDynamic))
              (:Finished
                (Rendering|Material|SetScalarParameterValue (Variables|Default|GetCrystalDynamicMaterial_03) "Transition" 1.0 :!class /Script/Engine.MaterialInstanceDynamic)
                (bind _highlightvalue_3 (Timeline|Timeline_2 PlayFromStart)
                  (:Update
                    (Rendering|Material|SetScalarParameterValue (Variables|Default|GetCrystalDynamicMaterial_03) "Highlight" _highlightvalue_3 :!class /Script/Engine.MaterialInstanceDynamic))))))))
      (:then_2
        (bind _returnvalue (Actor|GetActorOfClass "/Game/Art/Tools/HellDoor/BP_HellDoor.BP_HellDoor_C"))
        (Utilities|FlowControl|Delay 9.0)
        (Default|EndGameDoorAnimation _returnvalue))
      (:then_3
        ;;[0 0 0] WidgetEndGame
        (Utilities|FlowControl|Delay 11.5)
        (Game|SetGamePaused true)
        (bind _returnvalue_2 (UserInterface|CreateWidget "/Game/Widget/WB_Ending.WB_Ending_C"))
        (UserInterface|Viewport|AddtoViewport _returnvalue_2 0)))))

(fn ConstructionScript
  (bind _pivot_orbitingcrystal01 (Variables|Default|GetPivot_OrbitingCrystal01))
  (bind _pivot_orbitingcrystal02 (Variables|Default|GetPivot_OrbitingCrystal02))
  (bind _pivot_orbitingcrystal03 (Variables|Default|GetPivot_OrbitingCrystal03))
  (bind _relativerotation (Variables|/Script/Engine.SceneComponent|GetRelativeRotation _pivot_orbitingcrystal02))
  (bind _relativerotation_2 (Variables|/Script/Engine.SceneComponent|GetRelativeRotation _pivot_orbitingcrystal01))
  (bind _relativerotation_3 (Variables|/Script/Engine.SceneComponent|GetRelativeRotation _pivot_orbitingcrystal03))
  (Variables|Default|SetStartingLocation_Crystal (Variables|/Script/Engine.SceneComponent|GetRelativeLocation (Variables|Default|GetPivot_Crystal)))
  (Variables|Default|SetStartingLocation_OrbitingCrystal01 (Variables|/Script/Engine.SceneComponent|GetRelativeLocation (Variables|Default|GetPivot_OrbitingCrystal01)))
  (Variables|Default|SetStartingLocation_OrbitingCrystal02 (Variables|/Script/Engine.SceneComponent|GetRelativeLocation (Variables|Default|GetPivot_OrbitingCrystal02)))
  (Variables|Default|SetStartingLocation_OrbitingCrystal03 (Variables|/Script/Engine.SceneComponent|GetRelativeLocation (Variables|Default|GetPivot_OrbitingCrystal03)))
  (Variables|Default|SetStartingRotation_OrbitingCrystal01 (Math|Vector|MakeVector (.roll _relativerotation_2) (.pitch _relativerotation_2) (.yaw _relativerotation_2)))
  (Variables|Default|SetStartingRotation_OrbitingCrystal02 (Math|Vector|MakeVector (.roll _relativerotation) (.pitch _relativerotation) (.yaw _relativerotation)))
  (Variables|Default|SetStartingRotation_OrbitingCrystal03 (Math|Vector|MakeVector (.roll _relativerotation_3) (.pitch _relativerotation_3) (.yaw _relativerotation_3)))
  (Rendering|Material|SetMaterial (Variables|Default|GetSM_GroundPattern) 0 "/Game/Art/FX/Environmentals/ArenaCrystal/M_GroundPattern_Corrupt.M_GroundPattern_Corrupt"))