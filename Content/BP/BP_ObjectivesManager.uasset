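; Objectives manager that drives the on-screen objectives widget as the player progresses through the pre-arena, religious corridor and arena stages.
; After a startup delay, it finds the WB_Objectives widget and binds to events on fence doors, arena entry doors and Forge, Magic and Jail spawners, found by class and tag.
; Spawner completions tick individual objectives, while stage changes use timed delays to slide the list out and show the next set.
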(event `self.ReceiveBeginPlay`
  (`KismetSystemLibrary.Delay` 6.0)
  (bind _foundwidgets (`WidgetBlueprintLibrary.GetAllWidgetsOfClass` "/Game/Widget/WB_Objectives.WB_Objectives_C"))
  (for _array_element _foundwidgets
    (set `self.Widget_Objectives` _array_element))
  (`GameplayStatics.GetAllActorsOfClassWithTag` null)
  (bind _outactors (`GameplayStatics.GetAllActorsOfClass` "/Game/BP/Doors/FenceDoorCorridor02/BP_FenceDoor.BP_FenceDoor_C"))
  (for _array_element_2 _outactors
    (add `/Game/BP/Doors/FenceDoorCorridor02/BP_FenceDoor.DoorIsOpening` _array_element_2 (delegate `PreArenaObjectivesAppearance`)))
  (bind _outactors_2 (`GameplayStatics.GetAllActorsOfClassWithTag` "/Game/BP/Doors/DoorEntryArena/BP_DoorEntryArena.BP_DoorEntryArena_C" "DoorPreArena"))
  (for _array_element_3 _outactors_2
    (add `/Game/BP/Doors/DoorEntryArena/BP_DoorEntryArena.PreArenaSpawnerFinished` _array_element_3 (delegate `CorridorObjectivesAppearance`)))
  (bind _outactors_3 (`GameplayStatics.GetAllActorsOfClassWithTag` "/Game/BP/Doors/DoorEntryArena/BP_DoorEntryArena.BP_DoorEntryArena_C" "DoorArena"))
  (for _array_element_4 _outactors_3
    (add `/Game/BP/Doors/DoorEntryArena/BP_DoorEntryArena.ArenaSpawnerStarted` _array_element_4 (delegate `ArenaObjectivesAppearance`)))
  (bind _outactors_4 (`GameplayStatics.GetAllActorsOfClassWithTag` "/Game/BP/Spawner/BP_MultiAreaSpawner.BP_MultiAreaSpawner_C" "Forge"))
  (for _array_element_5 _outactors_4
    (add `MultiAreaSpawner.OnSpawnerFinished` _array_element_5 (delegate `ForgeObjectifClear`)))
  (bind _outactors_5 (`GameplayStatics.GetAllActorsOfClassWithTag` "/Game/BP/Spawner/BP_MultiAreaSpawner.BP_MultiAreaSpawner_C" "Magic"))
  (for _array_element_6 _outactors_5
    (add `MultiAreaSpawner.OnSpawnerFinished` _array_element_6 (delegate `MagicObjectifClear`)))
  (bind _outactors_6 (`GameplayStatics.GetAllActorsOfClassWithTag` "/Game/BP/Spawner/BP_MultiAreaSpawner.BP_MultiAreaSpawner_C" "Jail"))
  (for _array_element_7 _outactors_6
    (add `MultiAreaSpawner.OnSpawnerFinished` _array_element_7 (delegate `JailObjectifClear`))))

(event `PreArenaObjectivesAppearance`
  (bind _widget_objectives (`self.Widget_Objectives`))
  (`/Game/Widget/WB_Objectives.Objectif01_Completed` _widget_objectives)
  (`KismetSystemLibrary.Delay` 2.0)
  (`/Game/Widget/WB_Objectives.LeaveScreen` _widget_objectives)
  (`KismetSystemLibrary.Delay` 2.0)
  (`/Game/Widget/WB_Objectives.PreArena` _widget_objectives))

(event `ForgeObjectifClear`
  (`/Game/Widget/WB_Objectives.Objectif02_Completed` (`self.Widget_Objectives`)))

(event `MagicObjectifClear`
  (`/Game/Widget/WB_Objectives.Objectif03_Completed` (`self.Widget_Objectives`)))

(event `JailObjectifClear`
  (`/Game/Widget/WB_Objectives.Objectif01_Completed` (`self.Widget_Objectives`)))

(event `CorridorObjectivesAppearance`
  (bind _widget_objectives (`self.Widget_Objectives`))
  (`KismetSystemLibrary.Delay` 2.0)
  (`/Game/Widget/WB_Objectives.LeaveScreen` _widget_objectives)
  (`KismetSystemLibrary.Delay` 2.0)
  (`/Game/Widget/WB_Objectives.ReligiousCorridor` _widget_objectives))

(event `ArenaObjectivesAppearance`
  (bind _widget_objectives (`self.Widget_Objectives`))
  (`/Game/Widget/WB_Objectives.Objectif01_Completed` _widget_objectives)
  (`KismetSystemLibrary.Delay` 2.0)
  (`/Game/Widget/WB_Objectives.LeaveScreen` _widget_objectives)
  (`KismetSystemLibrary.Delay` 2.0)
  (`/Game/Widget/WB_Objectives.Arena` _widget_objectives))

(fn `UserConstructionScript`)