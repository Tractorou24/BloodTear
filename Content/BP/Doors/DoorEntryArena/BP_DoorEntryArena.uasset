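; Arena entry door that swings two leaves open and shut as the player enters and leaves its trigger, provided it is unlocked.
; On BeginPlay it binds to every BP_MultiAreaSpawner carrying the configured tag.
; A new wave blocks opening, and the door unlocks once the count of finished spawners equals the number found.
; Separate opening and closing timelines drive the door yaw, each stopping the other.
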(event `self.ReceiveBeginPlay`
  (bind _collisiontestanim (`self.CollisionTestAnim`))
  (add `PrimitiveComponent.OnComponentBeginOverlap` _collisiontestanim (delegate `OnComponentBeginOverlap_Event`))
  (add `PrimitiveComponent.OnComponentEndOverlap` _collisiontestanim (delegate `OnComponentEndOverlap_Event`))
  (bind _outactors (`GameplayStatics.GetAllActorsOfClassWithTag` "/Game/BP/Spawner/BP_MultiAreaSpawner.BP_MultiAreaSpawner_C" (`self.SpawnerTagCheck`)))
  (set `self.NumberOfSpawner` (`KismetArrayLibrary.Array_Length` _outactors))
  (for _array_element _outactors
    (add `MultiAreaSpawner.OnSpawnerFinished` _array_element (delegate `OnMainRoomSpawnerFinished`))
    (add `MultiAreaSpawner.OnNewWave` _array_element (delegate `OnNewWave`))))

(event `OnComponentBeginOverlap_Event`
  (params (OverlappedComponent :type "PrimitiveComponent Object Reference") (OtherActor :type "Actor Object Reference") (OtherComp :type "PrimitiveComponent Object Reference") (OtherBodyIndex :type Integer) (bFromSweep :type Boolean) (SweepResult :type "HitResult Structure (by ref)"))
  (if (`self.ActorHasTag` OtherActor "Player")
    (`self.OpenDoor`)))

(event `OnComponentEndOverlap_Event`
  (params (OverlappedComponent :type "PrimitiveComponent Object Reference") (OtherActor :type "Actor Object Reference") (OtherComp :type "PrimitiveComponent Object Reference") (OtherBodyIndex :type Integer))
  (if (`self.ActorHasTag` OtherActor "Player")
    (if (`self.isOpen?`)
      (`self.CloseDoor`))))

(event `OnMainRoomSpawnerFinished`
  (set `self.NumberSpawnerFinished` (+ (`self.NumberSpawnerFinished`) 1))
  (if (== (`self.NumberSpawnerFinished`) (`self.NumberOfSpawner`))
    (set `self.CanBeOpened` true)))

(event `OnNewWave`
  (params (WaveNumber :type Integer))
  (set `self.CanBeOpened` false))

(event `OpenDoor`
  (if (`self.CanBeOpened`)
    (set `self.isOpen?` true)
    (`|ExecutionSequence`
      (:`then_0`
        (bind (_direction _rotation) (`Timeline|DoorClosing` :!via `Stop` :!label _label)
          (:`Update`
            (`SceneComponent.K2_SetRelativeRotation` (`self.Door01`) (`KismetMathLibrary.MakeRotator` 0.0 0.0 _rotation) false false)
            (`SceneComponent.K2_SetRelativeRotation` (`self.Door02`) (`KismetMathLibrary.MakeRotator` 0.0 0.0 _rotation) false false))
          (:`Finished`
            (set `self.isOpen?` false))))
      (:`then_1`
        (bind (_direction_2 _rotation_2) (`Timeline|DoorOpening` :!via `SetNewTime` :!label _label_2)
          (:`Update`
            (`SceneComponent.K2_SetRelativeRotation` (`self.Door01`) (`KismetMathLibrary.MakeRotator` 0.0 0.0 _rotation_2) false false)
            (`SceneComponent.K2_SetRelativeRotation` (`self.Door02`) (`KismetMathLibrary.MakeRotator` 0.0 0.0 _rotation_2) false false))))
      (:`then_2`
        (goto _label_2)))))

(event `CloseDoor`
  (if (`self.isOpen?`)
    (`|ExecutionSequence`
      (:`then_0`
        (goto _label_2 :!via `Stop`))
      (:`then_1`
        (goto _label :!via `SetNewTime`))
      (:`then_2`
        (goto _label)))))

(fn `UserConstructionScript`)