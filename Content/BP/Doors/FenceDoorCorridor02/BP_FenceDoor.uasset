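; Fence door that slides along Z when the player character enters its TestingBox trigger.
; BeginPlay binds the box overlap, which plays the Opening timeline from the start to drive PivotPoint's relative Z location.
; The overlap unbinds only when the timeline finishes, so the door never closes, but re-entering mid-motion restarts the animation.
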(event `self.ReceiveBeginPlay`
  (add `PrimitiveComponent.OnComponentBeginOverlap` (`self.TestingBox`) (delegate `TestFenceOpening`)))

(event `TestFenceOpening`
  (params (OverlappedComponent :type "PrimitiveComponent Object Reference") (OtherActor :type "Actor Object Reference") (OtherComp :type "PrimitiveComponent Object Reference") (OtherBodyIndex :type Integer) (bFromSweep :type Boolean) (SweepResult :type "HitResult Structure (by ref)"))
  (if (== OtherActor (`GameplayStatics.GetPlayerCharacter` 0))
    (bind (_direction _translationz) (`Timeline|Opening` :!via `PlayFromStart`)
      (:`Update`
        (`SceneComponent.K2_SetRelativeLocation` (`self.PivotPoint`) (`KismetMathLibrary.MakeVector` 0.0 0.0 _translationz) false false))
      (:`Finished`
        (remove `PrimitiveComponent.OnComponentBeginOverlap` (`self.TestingBox`) (delegate `TestFenceOpening`))))))

(fn `UserConstructionScript`)