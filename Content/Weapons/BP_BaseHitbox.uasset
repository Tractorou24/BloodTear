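; BP_BaseHitbox is a base weapon hitbox that damages overlapping EnsEnemyBase enemies once each.
; An ability passes in damage, level and combo step through Initialize, which Tick asserts has run.
; Tick polls every shape component's overlaps, records new hits, applies BPGE_Damage via a SetByCaller spec from the avatar's ability system, then fires CallOnDamaging and the ability's knockback.
; A debug flag shows the shapes in game.
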(event `self.ReceiveBeginPlay`
  (set `self.Colliders` (`self.K2_GetComponentsByClass` "/Script/Engine.ShapeComponent"))
  (`SceneComponent.SetHiddenInGame` (`SceneComponent.GetChildComponent` (`self.DefaultSceneRoot`) 0) (not (`self.IsDebug`)) true))

(event `self.ReceiveTick`
  (params (DeltaSeconds :type "Float (single-precision)"))
  (`EnsBlueprintAssert.BlueprintAssert` self (`self.IsInitialized`))
  (for _array_element (`self.Colliders`)
    (bind (_arrayindex _arrayelement) (`/Engine/EditorBlueprintResources/StandardMacros.ReverseForEachLoop` (`PrimitiveComponent.GetOverlappingActors` _array_element "/Script/ENS.EnsEnemyBase"))
      (:`LoopBody`
        (bind _asens_enemy_base (cast `EnsEnemyBase` _arrayelement)
          (:`then`
            (if (not (`BlueprintSetLibrary.Set_Contains` (`self.Hits`) _asens_enemy_base))
              (`self.GiveDamage` _asens_enemy_base 1.0 (`self.Damage`))
              (`BlueprintSetLibrary.Set_Add` (`self.Hits`) _asens_enemy_base)
              (`self.OnDamaging` _asens_enemy_base)
              (`EnsGameplayAbilityBase.ApplyKnockback` (`self.Ability`) _asens_enemy_base (`KismetMathLibrary.Conv_IntToByte` (`self.Level`)) (`KismetMathLibrary.Conv_IntToByte` (`self.ComboStep`)))))
          (:`CastFailed`
            (`EnsBlueprintAssert.BlueprintAssert` self)))))))

(fn `GiveDamage`
  (params (Target :type "EnsCharacterBase Object Reference") (AttackLevel :type "Float (double-precision)") (Damage :type "Float (double-precision)"))
  (bind _returnvalue (`AbilitySystemBlueprintLibrary.GetAbilitySystemComponent` (`GameplayAbility.GetAvatarActorFromActorInfo` (`self.Ability`))))
  (bind _returnvalue_2 (`AbilitySystemBlueprintLibrary.AssignTagSetByCallerMagnitude` (`AbilitySystemComponent.MakeOutgoingSpec` _returnvalue "/Game/Characters/Player/Abilities/DevelopperTests/BPGE_Damage.BPGE_Damage_C" AttackLevel (`AbilitySystemComponent.MakeEffectContext` _returnvalue)) (struct :`TagName` "Ability.Damage") Damage))
  (`AbilitySystemComponent.BP_ApplyGameplayEffectSpecToSelf` (`AbilitySystemBlueprintLibrary.GetAbilitySystemComponent` Target) _returnvalue_2)
  (return))

(fn `Initialize`
  (params (Damage :type "Float (double-precision)") (Ability :type "EnsGameplayAbilityBase Object Reference") (Level :type Integer) (ComboStep :type Integer))
  (set `self.Damage` Damage)
  (set `self.Ability` Ability)
  (set `self.Level` Level)
  (set `self.ComboStep` ComboStep)
  (set `self.IsInitialized` true))

(fn `UserConstructionScript`)