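; Hit box actor for the third hit of the sword base attack, adding level-based slash trail VFX on spawn.
; After the parent BeginPlay and a short delay, it reads the player character's current level.
; It spawns one-shot Niagara trails at marker component transforms, with higher levels adding more trails and level-specific systems.
; The top level reuses one level-two trail alongside its own.
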(event `self.ReceiveBeginPlay`
  (bind _niagara_03 (`self.Niagara_03`))
  (bind _niagara_01 (`self.Niagara_01`))
  (bind _niagara_02 (`self.Niagara_02`))
  (bind _niagara_04 (`self.Niagara_04`))
  (bind _returnvalue (`SceneComponent.K2_GetComponentLocation` _niagara_02))
  (bind _returnvalue_2 (`SceneComponent.K2_GetComponentRotation` _niagara_03))
  (bind _returnvalue_3 (`SceneComponent.K2_GetComponentLocation` _niagara_01))
  (bind _returnvalue_4 (`SceneComponent.K2_GetComponentRotation` _niagara_01))
  (bind _returnvalue_5 (`SceneComponent.K2_GetComponentRotation` _niagara_02))
  (bind _returnvalue_6 (`SceneComponent.K2_GetComponentLocation` _niagara_03))
  (`parent.ReceiveBeginPlay`)
  (bind _asens_player_character (cast `EnsPlayerCharacter` (`GameplayStatics.GetPlayerCharacter` 0)))
  (`KismetSystemLibrary.Delay` 0.1)
  (bind _returnvalue_7 (`EnsPlayerCharacter.GetCurrentLevel` _asens_player_character))
  (if (== _returnvalue_7 1)
    (`NiagaraFunctionLibrary.SpawnSystemAtLocation` "/Game/Art/FX/Trail/Sword_Lvl1/NS_SwordTrailLvl1_03.NS_SwordTrailLvl1_03" _returnvalue_3 _returnvalue_4)
    (`NiagaraFunctionLibrary.SpawnSystemAtLocation` "/Game/Art/FX/Trail/Sword_Lvl1/NS_SwordTrailLvl1_03.NS_SwordTrailLvl1_03" _returnvalue _returnvalue_5)
    (elif (== _returnvalue_7 2)
      (`NiagaraFunctionLibrary.SpawnSystemAtLocation` "/Game/Art/FX/Trail/Sword_Lvl1/NS_SwordTrailLvl2_03.NS_SwordTrailLvl2_03" _returnvalue_3 _returnvalue_4)
      (`NiagaraFunctionLibrary.SpawnSystemAtLocation` "/Game/Art/FX/Trail/Sword_Lvl1/NS_SwordTrailLvl2_03.NS_SwordTrailLvl2_03" _returnvalue _returnvalue_5)
      (`NiagaraFunctionLibrary.SpawnSystemAtLocation` "/Game/Art/FX/Trail/Sword_Lvl1/NS_SwordTrailLvl2_04.NS_SwordTrailLvl2_04" _returnvalue_6 _returnvalue_2)
      (elif (== _returnvalue_7 3)
        (`NiagaraFunctionLibrary.SpawnSystemAtLocation` "/Game/Art/FX/Trail/Sword_Lvl1/NS_SwordTrailLvl3_03.NS_SwordTrailLvl3_03" _returnvalue_3 _returnvalue_4)
        (`NiagaraFunctionLibrary.SpawnSystemAtLocation` "/Game/Art/FX/Trail/Sword_Lvl1/NS_SwordTrailLvl3_03.NS_SwordTrailLvl3_03" _returnvalue _returnvalue_5)
        (`NiagaraFunctionLibrary.SpawnSystemAtLocation` "/Game/Art/FX/Trail/Sword_Lvl1/NS_SwordTrailLvl2_04.NS_SwordTrailLvl2_04" _returnvalue_6 _returnvalue_2)
        (`NiagaraFunctionLibrary.SpawnSystemAtLocation` "/Game/Art/FX/Trail/Sword_Lvl1/NS_SwordTrailLvl3_04.NS_SwordTrailLvl3_04" (`SceneComponent.K2_GetComponentLocation` _niagara_04) (`SceneComponent.K2_GetComponentRotation` _niagara_04))))))

(fn `UserConstructionScript`)