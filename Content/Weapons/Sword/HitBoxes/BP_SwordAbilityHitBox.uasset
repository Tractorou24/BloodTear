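; Moving hit box for a sword ability that travels forward and removes itself after a set distance.
; Each tick it offsets itself along local X at Speed, without sweep.
; Initialize passes damage and ability to the parent, then sets a timer that destroys the actor after Distance divided by Speed.
; The Level and ComboStep inputs are unused here.
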(event `self.ReceiveBeginPlay`
  (`parent.ReceiveBeginPlay`))

(event `self.ReceiveTick`
  (params (DeltaSeconds :type "Float (single-precision)"))
  (`parent.ReceiveTick` DeltaSeconds)
  (`self.K2_AddActorLocalOffset` (* DeltaSeconds (`KismetMathLibrary.MakeVector` (`self.Speed`)))))

(fn `Destroy`
  (`self.K2_DestroyActor`))

(fn `Initialize`
  (params (Damage :type "Float (double-precision)") (Ability :type "EnsGameplayAbilityBase Object Reference") (Level :type Integer) (ComboStep :type Integer))
  (`parent.Initialize` Damage Ability 0 0)
  (`KismetSystemLibrary.K2_SetTimer` null "Destroy" (/ (`self.Distance`) (`self.Speed`))))

(fn `UserConstructionScript`)