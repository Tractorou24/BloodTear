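; Hit box actor for the third dagger base attack, which spawns that attack's slash effect when it begins play.
; After a brief delay it reads the player character's current level and spawns the matching level 1, 2 or 3 Niagara system at its Niagara1 component's location and rotation.
; Despite the Lvl1 name, it covers all three levels, and the graph itself contains only this visual logic.
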(event `self.ReceiveBeginPlay`
  (bind _niagara1 (`self.Niagara1`))
  (bind _returnvalue (`SceneComponent.K2_GetComponentLocation` _niagara1))
  (bind _returnvalue_2 (`SceneComponent.K2_GetComponentRotation` _niagara1))
  (`parent.ReceiveBeginPlay`)
  (bind _asens_player_character (cast `EnsPlayerCharacter` (`GameplayStatics.GetPlayerCharacter` 0)))
  (`KismetSystemLibrary.Delay` 0.01)
  (bind _returnvalue_3 (`EnsPlayerCharacter.GetCurrentLevel` _asens_player_character))
  (if (== _returnvalue_3 1)
    (`NiagaraFunctionLibrary.SpawnSystemAtLocation` "/Game/Art/FX/Skills/Dagger/Dagger_Lvl/NS_AADaggerLvl1_03.NS_AADaggerLvl1_03" _returnvalue _returnvalue_2)
    (elif (== _returnvalue_3 2)
      (`NiagaraFunctionLibrary.SpawnSystemAtLocation` "/Game/Art/FX/Skills/Dagger/Dagger_Lvl/NS_AADaggerLvl2_03.NS_AADaggerLvl2_03" _returnvalue _returnvalue_2)
      (elif (== _returnvalue_3 3)
        (`NiagaraFunctionLibrary.SpawnSystemAtLocation` "/Game/Art/FX/Skills/Dagger/Dagger_Lvl/NS_AADaggerLvl3_03.NS_AADaggerLvl3_03" _returnvalue _returnvalue_2)))))

(fn `UserConstructionScript`)