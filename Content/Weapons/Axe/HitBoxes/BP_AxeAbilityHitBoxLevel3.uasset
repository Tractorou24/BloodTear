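; Level 3 hitbox for the axe ability, a child Blueprint that adds a visual effect on spawn.
; BeginPlay runs the parent logic, then spawns the NS_SkillAxe01_01 system at its Niagara component's world location and rotation.
; An unconnected leftover branch would pick a different trail or bubble effect from the player's current level after a short delay, but it never runs.
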(event `self.ReceiveBeginPlay`
  (bind _niagara (`self.Niagara`))
  (`parent.ReceiveBeginPlay`)
  (`NiagaraFunctionLibrary.SpawnSystemAtLocation` "/Game/Art/FX/Skills/Axe/NS_SkillAxe01_01.NS_SkillAxe01_01" (`SceneComponent.K2_GetComponentLocation` _niagara) (`SceneComponent.K2_GetComponentRotation` _niagara)))

(fn `UserConstructionScript`)